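; Trigger actor that unloads a streaming sublevel, named by LevelToUnload, when a DefaultCharacter overlaps its OverlapBox.
; The unload is non-blocking and is followed by a printed message naming the level.
; A chain of name checks then clears the character's matching presence flag for one of four Comm quadrant levels (West/East, North/South).
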(event OnComponentBeginOverlap(OverlapBox)
  (params (OverlappedComponent :type Primitive%20Component%20Object%20Reference) (OtherActor :type Actor%20Object%20Reference) (OtherComp :type Primitive%20Component%20Object%20Reference) (OtherBodyIndex :type Integer) (bFromSweep :type Boolean) (SweepResult :type Hit%20Result%20Structure%20%28by%20ref%29))
  (bind _leveltounload (Variables|Default|GetLevelToUnload))
  (bind _asdefault_character (Utilities|Casting|CastToDefaultCharacter OtherActor))
  (Game|UnloadStreamLevel(byName) _leveltounload false)
  (Development|PrintString (Utilities|String|Append (Utilities|String|ToString(Name) _leveltounload) "Unloaded"))
  (if (== _leveltounload "Comm_West_North")
    (Variables|/Game/Blueprints/SetUp/DefaultCharacter.DefaultCharacter_C|SetIn_CNW? _asdefault_character false)
    (elif (== _leveltounload "Comm_West_South")
      (Variables|/Game/Blueprints/SetUp/DefaultCharacter.DefaultCharacter_C|SetIn_CSW? _asdefault_character false)
      (elif (== _leveltounload "Comm_East_North")
        (Variables|/Game/Blueprints/SetUp/DefaultCharacter.DefaultCharacter_C|SetIn_CNE? _asdefault_character false)
        (elif (== _leveltounload "Comm_East_South")
          (Variables|/Game/Blueprints/SetUp/DefaultCharacter.DefaultCharacter_C|SetIn_CSE? _asdefault_character false))))))

(fn ConstructionScript)