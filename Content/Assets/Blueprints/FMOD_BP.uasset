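; An FMOD sound emitter actor that plays its audio component on BeginPlay and simulates occlusion between itself and the player pawn.
; When occlusion is enabled, Tick uses a Delay to throttle updates to UpdateRate and measures distance to a point raised above the pawn's origin.
; Within MaxDistance, a debug-drawn multi-object trace against WorldStatic scales the hit count by a per-hit percentage into an audio parameter, zeroed when unobstructed.
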(event EventBeginPlay
  (Class|FMODAudioComponent|Play (Variables|Default|GetAudioComponent))
  (Variables|Default|SetListener (Game|Player|GetPlayerPawn 0)))

(event EventTick
  (params (DeltaSeconds :type Float%20%28single-precision%29))
  (bind _audiocomponent (Variables|Default|GetAudioComponent))
  (bind _parametername (Variables|Default|GetParameterName))
  (if (Variables|Default|GetEnableOcclusion?)
    (Utilities|FlowControl|Delay (/ 1.0 (Variables|Default|GetUpdateRate)))
    (bind _distance (CallFunction|CalculatePositions (Transformation|GetActorLocation) (Transformation|GetActorLocation (Variables|Default|GetListener))))
    (bind _output_get (Variables|Default|SetDistance _distance))
    (if (<= _output_get (Variables|Default|GetMaxDistance))
      (bind (_outhits _returnvalue) (Class|KismetSystemLibrary|LineTraceMultiforObjects (Variables|Default|GetSource%20Location) (Variables|Default|GetListener%20Location) (Utilities|Array|MakeArray "ObjectTypeQuery1") false (Utilities|Array|MakeArray (Variables|Default|GetListener)) "ForOneFrame" true))
      (if _returnvalue
        (Class|FMODAudioComponent|SetParameter _audiocomponent _parametername (/ (* (Math|Conversions|ToFloat(Integer) (Utilities|Array|Length _outhits)) (Variables|Default|GetOcclusionPercentagePerHit)) 1e+02))
        (else
          (Class|FMODAudioComponent|SetParameter _audiocomponent _parametername 0.0))))))

(fn ConstructionScript)

(fn CalculatePositions
  (params (SourceLocation :type Vector) (ListenerLocation :type Vector))
  (bind _output_get (Variables|Default|SetListener%20Location (+ ListenerLocation "0,0,80.000000")))
  (bind _output_get_2 (Variables|Default|SetSource%20Location SourceLocation))
  (return (Math|Vector|VectorLength (- _output_get _output_get_2))))