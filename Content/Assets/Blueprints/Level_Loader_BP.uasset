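; Level loader trigger actor that moves the player to another level when the DefaultCharacter overlaps it.
; Before travel it saves Ultra Dynamic Sky's time of day to the FP82 game instance and clears its FirstLoad flag.
; It also stores the character's location as MainLocation in the "Main" level, or PavilionLocation otherwise, then opens LevelToLoad.
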(event EventBeginPlay)

(event Collision|EventActorBeginOverlap
  (params (OtherActor :type Actor%20Object%20Reference))
  (bind _asdefault_character (Utilities|Casting|CastToDefaultCharacter OtherActor))
  (Utilities|FlowControl|Sequence
    (:then_0
      (bind _asfp82game_instance (Utilities|Casting|CastToFP82GameInstance (Game|GetGameInstance)))
      (bind _returnvalue (Actor|GetActorOfClass "/Game/UltraDynamicSky/Blueprints/Ultra_Dynamic_Sky.Ultra_Dynamic_Sky_C"))
      (Variables|/Game/Assets/Blueprints/FP82GameInstance.FP82GameInstance_C|SetGlobalTime _asfp82game_instance (Variables|/Game/UltraDynamicSky/Blueprints/Ultra_Dynamic_Sky.Ultra_Dynamic_Sky_C|GetTime%20of%20Day _returnvalue))
      (Variables|/Game/Assets/Blueprints/FP82GameInstance.FP82GameInstance_C|SetFirstLoad? _asfp82game_instance false))
    (:then_1
      (bind _returnvalue_2 (Game|GetCurrentLevelName true))
      (if (Utilities|Enum|Equal(Enum) _returnvalue_2 "Main")
        (Variables|/Game/Assets/Blueprints/FP82GameInstance.FP82GameInstance_C|SetMainLocation _asfp82game_instance (Transformation|GetActorLocation _asdefault_character))
        (else
          (Variables|/Game/Assets/Blueprints/FP82GameInstance.FP82GameInstance_C|SetPavilion%20Location _asfp82game_instance (Transformation|GetActorLocation _asdefault_character)))))
    (:then_2
      (Game|OpenLevel(byObjectReference) (Variables|Default|GetLevelToLoad)))))

(event EventTick
  (params (DeltaSeconds :type Float%20%28single-precision%29)))

(fn ConstructionScript)