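; Low Worldkey kiosk actor that lets the player switch Horizons between its construction and built versions.
; BeginPlay picks the bottom widget from NumOptions, and actor overlap swaps the main screen between FC_Horizons_Full and Kiosk_WEDWAY.
; Sphere overlap toggles input, so keys 1 and 2 play a sound and asynchronously stream the matching levels in and out.
; Disconnected leftover chains include tag-based actor visibility toggles and a duplicate level swap.
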(event OnComponentBeginOverlap(Sphere)
  (params (OverlappedComponent :type Primitive%20Component%20Object%20Reference) (OtherActor :type Actor%20Object%20Reference) (OtherComp :type Primitive%20Component%20Object%20Reference) (OtherBodyIndex :type Integer) (bFromSweep :type Boolean) (SweepResult :type Hit%20Result%20Structure%20%28by%20ref%29))
  (Input|EnableInput (Game|GetPlayerController 0)))

(event OnComponentEndOverlap(Sphere)
  (params (OverlappedComponent :type Primitive%20Component%20Object%20Reference) (OtherActor :type Actor%20Object%20Reference) (OtherComp :type Primitive%20Component%20Object%20Reference) (OtherBodyIndex :type Integer))
  (Input|DisableInput (Game|GetPlayerController 0) 0))

(event EventBeginPlay
  (switch int (Variables|Default|GetNumOptions)
    (:Default
      (bind _returnvalue (UserInterface|CreateWidget "/Game/Assets/Widgets/FC_Bottom2.FC_Bottom2_C" 0 (Variables|Default|GetTexture%202D) :!label _label))
      (UserInterface|SetWidget (Variables|Default|GetWidget1) _returnvalue))
    (:2
      (goto _label))
    (:3
      (bind _returnvalue_2 (UserInterface|CreateWidget "/Game/Assets/Widgets/FC_Bottom3.FC_Bottom3_C" 0 (Variables|Default|GetTexture%202D)))
      (UserInterface|SetWidget (Variables|Default|GetWidget1) _returnvalue_2))
    (:6
      (UserInterface|SetWidget (Variables|Default|GetWidget1) 0))))

(event Collision|EventActorBeginOverlap
  (params (OtherActor :type Actor%20Object%20Reference))
  (bind _returnvalue (UserInterface|CreateWidget "/Game/Assets/Widgets/FC_Horizons_Full.FC_Horizons_Full_C"))
  (UserInterface|SetWidget (Variables|Default|GetWidget) _returnvalue))

(event EventTick
  (params (DeltaSeconds :type Float%20%28single-precision%29)))

(event Collision|EventActorEndOverlap
  (params (OtherActor :type Actor%20Object%20Reference))
  (bind _returnvalue (UserInterface|CreateWidget "/Game/Assets/Widgets/Kiosk_WEDWAY.Kiosk_WEDWAY_C"))
  (UserInterface|SetWidget (Variables|Default|GetWidget) _returnvalue)
  (bind _foundwidgets (Widget|GetAllWidgetsOfClass "/Game/Assets/Widgets/FC_Horizons_Full.FC_Horizons_Full_C" true))
  (Widget|RemovefromParent _foundwidgets))

(event Input|KeyboardEvents|1
  (params (Key :type Key%20Structure))
  (:Pressed
    (Audio|PlaySound2D "/Game/Assets/Audio/newworldkey.newworldkey" 1.0 1.0 0.0 0 0)
    (Class|GameplayStatics|LoadStreamLevelbySoftObjectPtr "/Game/Maps/FWE_Horizons_Construction.FWE_Horizons_Construction" true false)
    (Class|GameplayStatics|LoadStreamLevelbySoftObjectPtr "/Game/Maps/FWE_Horizons_Construction_Wall.FWE_Horizons_Construction_Wall" true false)
    (Class|GameplayStatics|UnloadStreamLevelbySoftObjectPtr "/Game/Maps/FWE_Horizons_Built.FWE_Horizons_Built" false)))

(event Input|KeyboardEvents|2
  (params (Key :type Key%20Structure))
  (:Pressed
    (Audio|PlaySound2D "/Game/Assets/Audio/newworldkey.newworldkey" 1.0 1.0 0.0 0 0)
    (Class|GameplayStatics|LoadStreamLevelbySoftObjectPtr "/Game/Maps/FWE_Horizons_Built.FWE_Horizons_Built" true false)
    (Class|GameplayStatics|UnloadStreamLevelbySoftObjectPtr "/Game/Maps/FWE_Horizons_Construction.FWE_Horizons_Construction" false)
    (Class|GameplayStatics|UnloadStreamLevelbySoftObjectPtr "/Game/Maps/FWE_Horizons_Construction_Wall.FWE_Horizons_Construction_Wall" false)))

(event Input|KeyboardEvents|3
  (params (Key :type Key%20Structure)))

(fn ConstructionScript)