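; DoorTest_BP is a test sliding door that opens and closes through overlaps on its Plane component.
; Begin overlap by an AnimateMe actor plays the DoorOpen sequence, while end overlap by a DefaultCharacter plays DoorClose.
; Both directions play the same sliding-door sound in 2D.
; OpenDoorEvent leads into the same open logic, and some leftover nodes are disconnected.
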(event OnComponentBeginOverlap(Plane)
  (params (OverlappedComponent :type Primitive%20Component%20Object%20Reference) (OtherActor :type Actor%20Object%20Reference) (OtherComp :type Primitive%20Component%20Object%20Reference) (OtherBodyIndex :type Integer) (bFromSweep :type Boolean) (SweepResult :type Hit%20Result%20Structure%20%28by%20ref%29))
  (Utilities|Casting|CastToAnimateMe OtherActor)
  (Sequencer|Player|Play (Variables|/Script/ActorSequence.ActorSequenceComponent|GetSequencePlayer (Variables|Default|GetDoorOpen)) :!class /Script/MovieScene.MovieSceneSequencePlayer)
  (Audio|PlaySound2D "/Game/Assets/Audio/slidingdooropen.slidingdooropen" 4.0 1.0 0.0 0 0))

(event OnComponentEndOverlap(Plane)
  (params (OverlappedComponent :type Primitive%20Component%20Object%20Reference) (OtherActor :type Actor%20Object%20Reference) (OtherComp :type Primitive%20Component%20Object%20Reference) (OtherBodyIndex :type Integer))
  (Utilities|Casting|CastToDefaultCharacter OtherActor)
  (Sequencer|Player|Play (Variables|/Script/ActorSequence.ActorSequenceComponent|GetSequencePlayer (Variables|Default|GetDoorClose)) :!class /Script/MovieScene.MovieSceneSequencePlayer)
  (Audio|PlaySound2D "/Game/Assets/Audio/slidingdooropen.slidingdooropen" 4.0 1.0 0.0 0 0))

(event Custom|OpenDoorEvent
  (Utilities|Casting|CastToAnimateMe (stale OnComponentBeginOverlap(Plane) OtherActor))
  (Sequencer|Player|Play (Variables|/Script/ActorSequence.ActorSequenceComponent|GetSequencePlayer (Variables|Default|GetDoorOpen)) :!class /Script/MovieScene.MovieSceneSequencePlayer)
  (Audio|PlaySound2D "/Game/Assets/Audio/slidingdooropen.slidingdooropen" 4.0 1.0 0.0 0 0))

(fn ConstructionScript)