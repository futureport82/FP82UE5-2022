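; Swinging gate actor that lets the player open an entrance labelled "Enter Futureport '82" with the Interact action.
; Overlapping its Plane component enables input for player 0 and shows a Press_Button prompt, without filtering which actor overlapped.
; Leaving disables input and removes every top-level Press_Button widget.
; Pressing Interact plays the actor's embedded ActorSequence animation and a 2D Newworldkey sound.
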(event OnComponentBeginOverlap(Plane)
  (params (OverlappedComponent :type Primitive%20Component%20Object%20Reference) (OtherActor :type Actor%20Object%20Reference) (OtherComp :type Primitive%20Component%20Object%20Reference) (OtherBodyIndex :type Integer) (bFromSweep :type Boolean) (SweepResult :type Hit%20Result%20Structure%20%28by%20ref%29))
  (Input|EnableInput (Game|GetPlayerController 0))
  (bind _returnvalue (UserInterface|CreateWidget "/Game/Assets/Widgets/Press_Button.Press_Button_C" (Game|GetPlayerController 0) "Enter Futureport '82"))
  (UserInterface|Viewport|AddtoViewport _returnvalue 0))

(event OnComponentEndOverlap(Plane)
  (params (OverlappedComponent :type Primitive%20Component%20Object%20Reference) (OtherActor :type Actor%20Object%20Reference) (OtherComp :type Primitive%20Component%20Object%20Reference) (OtherBodyIndex :type Integer))
  (Input|DisableInput 0)
  (bind _foundwidgets (Widget|GetAllWidgetsOfClass "/Game/Assets/Widgets/Press_Button.Press_Button_C" true))
  (Widget|RemovefromParent _foundwidgets))

(event EventBeginPlay)

(event Collision|EventActorBeginOverlap
  (params (OtherActor :type Actor%20Object%20Reference)))

(event EventTick
  (params (DeltaSeconds :type Float%20%28single-precision%29)))

(event Input|ActionEvents|InputActionInteract
  (params (Key :type Key%20Structure))
  (:Pressed
    (Sequencer|Player|Play (Variables|/Script/ActorSequence.ActorSequenceComponent|GetSequencePlayer (Variables|Default|GetActorSequence)) :!class /Script/MovieScene.MovieSceneSequencePlayer)
    (Audio|PlaySound2D "/Game/Assets/Audio/newworldkey.newworldkey" 0.4 1.0 0.0 0 0)))

(fn ConstructionScript)