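; Low_Worldkey_Seas_BP is an interactive kiosk actor for the Seas that shows UI through two widget components.
; On BeginPlay, NumOptions selects the FC_Bottom2 or FC_Bottom3 widget for Widget1, defaulting to FC_Bottom2, while six options sets it empty.
; Beginning an overlap enables player input and shows FC_Seas_Full on Widget.
; Ending it disables input, restores Kiosk_WEDWAY and attempts to remove top-level FC_Seas_Full widgets.
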(event EventBeginPlay
  (switch int (Variables|Default|GetNumOptions)
    (:Default
      (bind _returnvalue (UserInterface|CreateWidget "/Game/Assets/Widgets/FC_Bottom2.FC_Bottom2_C" 0 (Variables|Default|GetTexture%202D) :!label _label))
      (UserInterface|SetWidget (Variables|Default|GetWidget1) _returnvalue))
    (:2
      (goto _label))
    (:3
      (bind _returnvalue_2 (UserInterface|CreateWidget "/Game/Assets/Widgets/FC_Bottom3.FC_Bottom3_C" 0 (Variables|Default|GetTexture%202D)))
      (UserInterface|SetWidget (Variables|Default|GetWidget1) _returnvalue_2))
    (:6
      (UserInterface|SetWidget (Variables|Default|GetWidget1) 0))))

(event Collision|EventActorBeginOverlap
  (params (OtherActor :type Actor%20Object%20Reference))
  (Input|EnableInput (Game|GetPlayerController 0))
  (bind _returnvalue (UserInterface|CreateWidget "/Game/Assets/Widgets/FC_Seas_Full.FC_Seas_Full_C"))
  (UserInterface|SetWidget (Variables|Default|GetWidget) _returnvalue))

(event EventTick
  (params (DeltaSeconds :type Float%20%28single-precision%29)))

(event Collision|EventActorEndOverlap
  (params (OtherActor :type Actor%20Object%20Reference))
  (Input|DisableInput (Game|GetPlayerController 0))
  (bind _returnvalue (UserInterface|CreateWidget "/Game/Assets/Widgets/Kiosk_WEDWAY.Kiosk_WEDWAY_C"))
  (UserInterface|SetWidget (Variables|Default|GetWidget) _returnvalue)
  (bind _foundwidgets (Widget|GetAllWidgetsOfClass "/Game/Assets/Widgets/FC_Seas_Full.FC_Seas_Full_C" true))
  (Widget|RemovefromParent _foundwidgets))

(fn ConstructionScript)