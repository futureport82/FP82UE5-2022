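; Low WorldKey kiosk actor that lets the player switch between three states of the tagged RC tube actors.
; BeginPlay fills the lower widget with a two- or three-option panel based on NumOptions, or clears it for six.
; Overlap enables input and shows the FC_COMM_Full screen; leaving disables input and restores Kiosk_WEDWAY.
; Keys 1–3 play a sound and show original, alternate or off tubes by toggling actor visibility per tag.
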(event EventBeginPlay
  (switch int (Variables|Default|GetNumOptions)
    (:Default
      (bind _returnvalue (UserInterface|CreateWidget "/Game/Assets/Widgets/FC_Bottom2.FC_Bottom2_C" 0 (Variables|Default|GetTexture%202D) :!label _label))
      (UserInterface|SetWidget (Variables|Default|GetWidget1) _returnvalue))
    (:2
      (goto _label))
    (:3
      (bind _returnvalue_2 (UserInterface|CreateWidget "/Game/Assets/Widgets/FC_Bottom3.FC_Bottom3_C" 0 (Variables|Default|GetTexture%202D)))
      (UserInterface|SetWidget (Variables|Default|GetWidget1) _returnvalue_2))
    (:6
      (UserInterface|SetWidget (Variables|Default|GetWidget1) 0))))

(event Collision|EventActorBeginOverlap
  (params (OtherActor :type Actor%20Object%20Reference))
  (Input|EnableInput (Game|GetPlayerController 0))
  (bind _returnvalue (UserInterface|CreateWidget "/Game/Assets/Widgets/FC_COMM_Full.FC_COMM_Full_C"))
  (UserInterface|SetWidget (Variables|Default|GetWidget) _returnvalue))

(event EventTick
  (params (DeltaSeconds :type Float%20%28single-precision%29)))

(event Collision|EventActorEndOverlap
  (params (OtherActor :type Actor%20Object%20Reference))
  (Input|DisableInput (Game|GetPlayerController 0))
  (bind _returnvalue (UserInterface|CreateWidget "/Game/Assets/Widgets/Kiosk_WEDWAY.Kiosk_WEDWAY_C"))
  (UserInterface|SetWidget (Variables|Default|GetWidget) _returnvalue)
  (bind _foundwidgets (Widget|GetAllWidgetsOfClass "/Game/Assets/Widgets/FC_COMM_Full.FC_COMM_Full_C" true))
  (Widget|RemovefromParent _foundwidgets))

(event Input|KeyboardEvents|1
  (params (Key :type Key%20Structure))
  (:Pressed
    (Audio|PlaySound2D "/Game/Assets/Audio/newworldkey.newworldkey" 1.0 1.0 0.0 0 0)
    (Utilities|FlowControl|Sequence
      (:then_0
        (bind _outactors (Actor|GetAllActorswithTag "OriginalRCTubes"))
        (Rendering|SetActorHiddenInGame _outactors false))
      (:then_1
        (bind _outactors_2 (Actor|GetAllActorswithTag "RCTubes"))
        (Rendering|SetActorHiddenInGame _outactors_2 true))
      (:then_2
        (bind _outactors_3 (Actor|GetAllActorswithTag "RCTubesOff"))
        (Rendering|SetActorHiddenInGame _outactors_3 true)))))

(event Input|KeyboardEvents|2
  (params (Key :type Key%20Structure))
  (:Pressed
    (Audio|PlaySound2D "/Game/Assets/Audio/newworldkey.newworldkey" 1.0 1.0 0.0 0 0)
    (Utilities|FlowControl|Sequence
      (:then_0
        (bind _outactors (Actor|GetAllActorswithTag "OriginalRCTubes"))
        (Rendering|SetActorHiddenInGame _outactors true))
      (:then_1
        (bind _outactors_2 (Actor|GetAllActorswithTag "RCTubes"))
        (Rendering|SetActorHiddenInGame _outactors_2 false))
      (:then_2
        (bind _outactors_3 (Actor|GetAllActorswithTag "RCTubesOff"))
        (Rendering|SetActorHiddenInGame _outactors_3 true)))))

(event Input|KeyboardEvents|3
  (params (Key :type Key%20Structure))
  (:Pressed
    (Audio|PlaySound2D "/Game/Assets/Audio/newworldkey.newworldkey" 1.0 1.0 0.0 0 0)
    (Utilities|FlowControl|Sequence
      (:then_0
        (bind _outactors (Actor|GetAllActorswithTag "RCTubes"))
        (Rendering|SetActorHiddenInGame _outactors true))
      (:then_1
        (bind _outactors_2 (Actor|GetAllActorswithTag "OriginalRCTubes"))
        (Rendering|SetActorHiddenInGame _outactors_2 true))
      (:then_2
        (bind _outactors_3 (Actor|GetAllActorswithTag "RCTubesOff"))
        (Rendering|SetActorHiddenInGame _outactors_3 false)))))

(fn ConstructionScript)