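; WEDWAY ride car that reacts to TrackTrigger_BP volumes it overlaps along the track.
; Each trigger's TrackEvent starts or fades narration and background music, or loads FWE/FWW areas when the game instance flags a WEDWAY or Monorail ride.
; Its TrainMode then drives the vehicle train's speed, idle noise volume and door state.
; A timeline slides both doors apart and reverses to close them.
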(event OnComponentBeginOverlap(TriggerCollision)
  (params (OverlappedComponent :type Primitive%20Component%20Object%20Reference) (OtherActor :type Actor%20Object%20Reference) (OtherComp :type Primitive%20Component%20Object%20Reference) (OtherBodyIndex :type Integer) (bFromSweep :type Boolean) (SweepResult :type Hit%20Result%20Structure%20%28by%20ref%29))
  (bind _returnvalue (Game|GetGameInstance))
  (bind _narrationbgm (Variables|Default|GetNarrationBGM))
  (bind _narrationbgm_2 (Variables|Default|GetNarrationBGM))
  (bind _narrationbgm_3 (Variables|Default|GetNarrationBGM))
  (bind _astrack_trigger_bp (Utilities|Casting|CastToTrackTrigger_BP OtherActor))
  (Utilities|FlowControl|Sequence
    (:then_0
      (switch Utilities|FlowControl|Switch|SwitchonETrackTrigger (Variables|/Game/Blueprints/TrackTrigger_BP.TrackTrigger_BP_C|GetTrackEvent _astrack_trigger_bp)
        (:Narration
          (Audio|Components|Audio|SetSound (Variables|Default|GetNarrationAudio) (Variables|/Game/Blueprints/TrackTrigger_BP.TrackTrigger_BP_C|GetWEDWAYNarration _astrack_trigger_bp))
          (Audio|Components|Audio|FadeOut _narrationbgm 1.0 0.0 "Linear" :!class /Script/Engine.AudioComponent)
          (Audio|Components|Audio|SetSound _narrationbgm (Variables|/Game/Blueprints/TrackTrigger_BP.TrackTrigger_BP_C|GetWEDWAYBGM _astrack_trigger_bp))
          (Audio|Components|Audio|Play (Variables|Default|GetNarrationAudio) 0.0)
          (Audio|Components|Audio|SetVolumeMultiplier _narrationbgm_2 (Variables|/Game/Blueprints/TrackTrigger_BP.TrackTrigger_BP_C|GetWEDWAYBGMVolume _astrack_trigger_bp) :!class /Script/Engine.AudioComponent)
          (Audio|Components|Audio|FadeIn _narrationbgm_2 0.5 (Variables|/Game/Blueprints/TrackTrigger_BP.TrackTrigger_BP_C|GetWEDWAYBGMVolume _astrack_trigger_bp) 0.0 "Linear" :!class /Script/Engine.AudioComponent)
          (Audio|Components|Audio|Play (Variables|Default|GetNarrationBGM) (Variables|/Game/Blueprints/TrackTrigger_BP.TrackTrigger_BP_C|GetWEDWAYBGMStart _astrack_trigger_bp)))
        (:StopNarration
          (Audio|Components|Audio|FadeOut (Variables|Default|GetNarrationAudio) 1.5 0.0 "Linear" :!class /Script/Engine.AudioComponent))
        (:StartBGM
          (Audio|Components|Audio|SetSound _narrationbgm_3 (Variables|/Game/Blueprints/TrackTrigger_BP.TrackTrigger_BP_C|GetWEDWAYBGM _astrack_trigger_bp))
          (Audio|Components|Audio|FadeIn _narrationbgm_3 1.5 (Variables|/Game/Blueprints/TrackTrigger_BP.TrackTrigger_BP_C|GetWEDWAYBGMVolume _astrack_trigger_bp) 0.0 "Linear" :!class /Script/Engine.AudioComponent)
          (Audio|Components|Audio|Play _narrationbgm_3 (Variables|/Game/Blueprints/TrackTrigger_BP.TrackTrigger_BP_C|GetWEDWAYBGMStart _astrack_trigger_bp)))
        (:EndBGM
          (Audio|Components|Audio|FadeOut _narrationbgm_3 2.0 0.0 "Linear" :!class /Script/Engine.AudioComponent))
        (:LoadFWE
          (bind _asfp82game_instance (Utilities|Casting|CastToFP82GameInstance _returnvalue))
          (if (or (Variables|/Game/Assets/Blueprints/FP82GameInstance.FP82GameInstance_C|GetRiding%20WEDWAY _asfp82game_instance) (Variables|/Game/Assets/Blueprints/FP82GameInstance.FP82GameInstance_C|GetRiding%20Monorail _asfp82game_instance))
            (bind _returnvalue_2 (Actor|GetActorOfClass "/Game/FWE_Unload_FWW_Blueprint.FWE_Unload_FWW_Blueprint_C"))
            (Utilities|IsValid _returnvalue_2
              (:Is%20Valid
                (Default|LoadFWEBase _returnvalue_2)))))
        (:LoadFWW
          (bind _asfp82game_instance_2 (Utilities|Casting|CastToFP82GameInstance _returnvalue))
          (if (or (Variables|/Game/Assets/Blueprints/FP82GameInstance.FP82GameInstance_C|GetRiding%20WEDWAY _asfp82game_instance_2) (Variables|/Game/Assets/Blueprints/FP82GameInstance.FP82GameInstance_C|GetRiding%20Monorail _asfp82game_instance_2))
            (bind _returnvalue_3 (Actor|GetActorOfClass "/Game/FWW_Unload_FWE_Blueprint.FWW_Unload_FWE_Blueprint_C"))
            (Utilities|IsValid _returnvalue_3
              (:Is%20Valid
                (Default|LoadFWWBase _returnvalue_3)))))))
    (:then_1
      (switch Utilities|FlowControl|Switch|SwitchonETrainMode (Variables|/Game/Blueprints/TrackTrigger_BP.TrackTrigger_BP_C|GetTrainMode _astrack_trigger_bp)
        (:Idle
          (Audio|Components|Audio|SetVolumeMultiplier (Variables|Default|GetIdleNoise) 0.2 :!class /Script/Engine.AudioComponent)
          (Default|ChangeSpeed (Variables|Default|GetVehicleTrain) (Variables|/Game/Blueprints/TrackTrigger_BP.TrackTrigger_BP_C|GetTrainMode _astrack_trigger_bp) (Variables|/Game/Blueprints/TrackTrigger_BP.TrackTrigger_BP_C|GetSpeedScalar _astrack_trigger_bp) :!label _label))
        (:Travel
          (Audio|Components|Audio|SetVolumeMultiplier (Variables|Default|GetIdleNoise) 0.5 :!class /Script/Engine.AudioComponent)
          (goto _label))
        (:Loading
          (Audio|Components|Audio|SetVolumeMultiplier (Variables|Default|GetIdleNoise) 0.25 :!class /Script/Engine.AudioComponent)
          (goto _label))
        (:DoorOpen
          (CallFunction|DoorFunctionality true))
        (:DoorClose
          (CallFunction|DoorFunctionality false))
        (:SpeedScalar
          (goto _label))))))

(event Custom|DoorFunctionality
  (params (Open :type Boolean))
  (if Open
    (bind _newtrack_0 (Timeline|DoorOpenClose PlayFromStart)
      (:Update
        (Utilities|FlowControl|Sequence
          (:then_0
            (Transformation|SetRelativeLocation (Variables|Default|GetWEDWAY_Car_Master_Door_Left) (Math|Vector|MakeVector (* (* _newtrack_0 36.0) -1.0) 0.0 0.0) false false))
          (:then_1
            (Transformation|SetRelativeLocation (Variables|Default|GetWEDWAY_Car_Master_Door_Right) (Math|Vector|MakeVector (* _newtrack_0 36.0) 0.0 0.0) false false)))))
    (else
      (Timeline|DoorOpenClose ReverseFromEnd))))

(fn ConstructionScript)