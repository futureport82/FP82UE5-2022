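; Player character for a walkthrough-style world, combining movement, mouse look and run with scene navigation hotkeys.
; Input actions open options, teleport and held help widgets, load other levels or quit, while Relocate moves the player to the game instance's saved location.
; Time keys step SunSky's SolarTime by half hours, swapping streamed day and night lighting levels on exact matches at morning and evening thresholds.
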(event Custom|Relocate
  (bind _asfp82game_instance (Utilities|Casting|CastToFP82GameInstance (Game|GetGameInstance)))
  (Transformation|SetActorLocation (Variables|/Game/Assets/Blueprints/FP82GameInstance.FP82GameInstance_C|GetLastLocation _asfp82game_instance) false false))

(event EventBeginPlay
  (Variables|/Script/Engine.CharacterMovementComponent|SetMaxWalkSpeed (Variables|Character|GetCharacterMovement) 275.0))

(event Collision|EventActorBeginOverlap
  (params (OtherActor :type Actor%20Object%20Reference)))

(event Input|ActionEvents|InputActionRun
  (params (Key :type Key%20Structure))
  (:Pressed
    (Variables|/Script/Engine.CharacterMovementComponent|SetMaxWalkSpeed (Variables|Character|GetCharacterMovement) 1.5e+03))
  (:Released
    (Variables|/Script/Engine.CharacterMovementComponent|SetMaxWalkSpeed (Variables|Character|GetCharacterMovement) 275.0)))

(event Input|ActionEvents|InputActionEscapeMenu
  (params (Key :type Key%20Structure))
  (:Pressed
    (Game|QuitGame 0 "Quit" false)))

(event Input|ActionEvents|InputActionMap
  (params (Key :type Key%20Structure))
  (bind _returnvalue (Game|GetPlayerController 0))
  (:Pressed
    (Game|SetGamePaused false)
    (Variables|/Script/Engine.PlayerController|SetbShowMouseCursor _returnvalue true)
    (bind _returnvalue_2 (UserInterface|CreateWidget "/Game/Assets/Widgets/Teleport_Menu.Teleport_Menu_C" _returnvalue))
    (UserInterface|Viewport|AddtoViewport _returnvalue_2 0)))

(event Input|ActionEvents|InputActionOptions
  (params (Key :type Key%20Structure))
  (bind _returnvalue (Game|GetPlayerController 0))
  (:Pressed
    (Game|SetGamePaused true)
    (Variables|/Script/Engine.PlayerController|SetbShowMouseCursor _returnvalue true)
    (bind _returnvalue_2 (UserInterface|CreateWidget "/Game/Assets/Widgets/Scale_Test.Scale_Test_C" _returnvalue))
    (UserInterface|Viewport|AddtoViewport _returnvalue_2 0)))

(event Input|ActionEvents|InputActionMoveTimeForward
  (params (Key :type Key%20Structure))
  (:Pressed
    (bind _returnvalue (Actor|GetActorOfClass "/SunPosition/SunSky.SunSky_C"))
    (Utilities|FlowControl|Sequence
      (:then_0
        (if (>= (Variables|/SunPosition/SunSky.SunSky_C|GetSolarTime _returnvalue) 24.0)
          (Variables|/SunPosition/SunSky.SunSky_C|SetSolarTime _returnvalue 0.0)
          (else
            (Variables|/SunPosition/SunSky.SunSky_C|SetSolarTime _returnvalue (+ (Variables|/SunPosition/SunSky.SunSky_C|GetSolarTime _returnvalue) 0.5)))))
      (:then_1
        (if (== (Variables|/SunPosition/SunSky.SunSky_C|GetSolarTime _returnvalue) 19.0)
          (Game|UnloadStreamLevel(byName) "JII_Daylight" false)
          (Game|LoadStreamLevel(byName) "JIINightLights" true)
          (Variables|Default|SetDay? false)))
      (:then_2
        (if (== (Variables|/SunPosition/SunSky.SunSky_C|GetSolarTime _returnvalue) 6.5)
          (Game|UnloadStreamLevel(byName) "JIINightLights" false)
          (Game|LoadStreamLevel(byName) "JII_Daylight" true)
          (Variables|Default|SetDay? true))))))

(event Input|ActionEvents|InputActionMoveTimeBackward
  (params (Key :type Key%20Structure))
  (:Pressed
    (bind _returnvalue (Actor|GetActorOfClass "/SunPosition/SunSky.SunSky_C"))
    (Utilities|FlowControl|Sequence
      (:then_0
        (if (<= (Variables|/SunPosition/SunSky.SunSky_C|GetSolarTime _returnvalue) 0.0)
          (Variables|/SunPosition/SunSky.SunSky_C|SetSolarTime _returnvalue 24.0)
          (else
            (Variables|/SunPosition/SunSky.SunSky_C|SetSolarTime _returnvalue (- (Variables|/SunPosition/SunSky.SunSky_C|GetSolarTime _returnvalue) 0.5)))))
      (:then_1
        (if (== (Variables|/SunPosition/SunSky.SunSky_C|GetSolarTime _returnvalue) 19.0)
          (Game|UnloadStreamLevel(byName) "JIINightLights" false)
          (Game|LoadStreamLevel(byName) "JII_Daylight" true)
          (Variables|Default|SetDay? true)
          (Development|PrintString "SWITCH")))
      (:then_2
        (if (== (Variables|/SunPosition/SunSky.SunSky_C|GetSolarTime _returnvalue) 6.5)
          (Game|UnloadStreamLevel(byName) "JII_Daylight" false)
          (Game|LoadStreamLevel(byName) "JIINightLights" true)
          (Variables|Default|SetDay? false)
          (Development|PrintString "SWITCH"))))))

(event Input|ActionEvents|InputActionOpenLand
  (params (Key :type Key%20Structure))
  (:Pressed
    (Game|OpenLevel(byObjectReference) "/Game/Maps/Land_Master.Land_Master")))

(event Input|ActionEvents|InputActionOpenJii
  (params (Key :type Key%20Structure))
  (:Pressed
    (Game|OpenLevel(byObjectReference) "/Game/Maps/NewJIIMaster.NewJIIMaster")))

(event Input|ActionEvents|InputActionResetMap
  (params (Key :type Key%20Structure))
  (:Pressed
    (Game|OpenLevel(byObjectReference) "/Game/Maps/Main.Main")))

(event Input|ActionEvents|InputActionHelpToggle
  (params (Key :type Key%20Structure))
  (:Pressed
    (bind _returnvalue (UserInterface|CreateWidget "/Game/Assets/Widgets/DevHelpMenu.DevHelpMenu_C"))
    (UserInterface|Viewport|AddtoViewport _returnvalue 0))
  (:Released
    (Widget|RemovefromParent _returnvalue)))

(event Input|AxisEvents|InputAxisMoveForward
  (params (AxisValue :type Float%20%28single-precision%29))
  (Pawn|Input|AddMovementInput (Math|Vector|GetForwardVector (Transformation|GetActorRotation)) (* AxisValue 4.0) false))

(event Input|AxisEvents|InputAxisMoveRight
  (params (AxisValue :type Float%20%28single-precision%29))
  (Pawn|Input|AddMovementInput (Math|Vector|GetRightVector (Transformation|GetActorRotation)) (* AxisValue 1.0) false))

(event Input|AxisEvents|InputAxisTurn
  (params (AxisValue :type Float%20%28single-precision%29))
  (Pawn|Input|AddControllerYawInput (* AxisValue (Variables|Default|GetMouseSensitivity))))

(event Input|AxisEvents|InputAxisLookUp
  (params (AxisValue :type Float%20%28single-precision%29))
  (Pawn|Input|AddControllerPitchInput (* AxisValue (Variables|Default|GetMouseSensitivity))))

(fn ConstructionScript)