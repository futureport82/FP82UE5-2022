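; Teleport system Blueprint that moves player 0's pawn to one of the predefined TeleportSpots, chosen by index, behind a screen blackout.
; TeleportToSpot creates a BlackOutWidget and fades it in, then timed Sequence branches teleport the pawn mid-blackout, fade out and remove the widget.
; Control rotation comes from the spot's root transform, while the pawn's rotation is zeroed.
; A Teleporting flag ignores new requests until the transition finishes.
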(event Custom|TeleportToSpot
  (params (LocationI :type Integer))
  (bind _teleportspots (Variables|Default|GetTeleportSpots))
  (bind _output (Utilities|Array|Get(acopy) _teleportspots LocationI))
  (bind _defaultsceneroot (Variables|/Game/Blueprints/TeleportSpot_BP.TeleportSpot_BP_C|GetDefaultSceneRoot _output))
  (bind _returnvalue (Transformation|GetWorldTransform _defaultsceneroot))
  (if (not (Variables|Default|GetTeleporting))
    (Utilities|FlowControl|Sequence
      (:then_0
        (Variables|Default|SetTeleporting true))
      (:then_1
        ;[1 1 1] Black Out Widget Start
        (Utilities|FlowControl|Sequence
          (:then_0
            (bind _returnvalue_2 (UserInterface|CreateWidget "/Game/Blueprints/BlackOutWIdget.BlackOutWidget_C" (Game|GetPlayerController 0)))
            (Variables|Default|SetBlackOutWidget _returnvalue_2))
          (:then_1
            (UserInterface|Viewport|AddtoViewport (Variables|Default|GetBlackOutWidget) 0))
          (:then_2
            (Default|FadeToggle (Variables|Default|GetBlackOutWidget) true))))
      (:then_2
        ;[1 1 1] Teleport
        (Utilities|FlowControl|Delay 0.5)
        (Transformation|Teleport (Game|Player|GetPlayerPawn 0) (.location _returnvalue) "0, 0, 0")
        (Pawn|SetControlRotation (Game|GetPlayerController 0) (.rotation _returnvalue)))
      (:then_3
        ;[1 1 1] Black out Widget fade out
        (Utilities|FlowControl|Delay 1.0)
        (Default|FadeToggle (Variables|Default|GetBlackOutWidget) false)
        (Utilities|FlowControl|Delay 1.0)
        (Widget|RemovefromParent (Variables|Default|GetBlackOutWidget))
        (Variables|Default|SetTeleporting false)))))

(fn ConstructionScript)