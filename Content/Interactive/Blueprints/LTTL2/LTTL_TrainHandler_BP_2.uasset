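; Ride manager for the LTTL WEDway trains that spawns them evenly along a track spline and lets the player ride.
; Tick finds a train at the LTTL_Overlap zone and the car overlapping the player, then shows a ride prompt.
; SwitchToFirstPerson toggles riding, blending to a seat-attached camera driven by control-rotation deltas, or teleporting back to a fixed exit.
; Train, car and seat switching events are empty, their logic disconnected.
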(event Custom|SwitchToFirstPerson
  (params (TransitionTime :type Float%20%28single-precision%29))
  (CallFunction|ToggleWedwayView (Variables|Default|GetTrainNum) (Variables|Default|GetCarNum) TransitionTime true))

(event Custom|ChangeTrain)

(event Custom|ChangeCar)

(event Custom|SwitchSitting)

(event EventBeginPlay
  (for _index (range 0 (- (Variables|Default|GetTrainsAmount) 1))
    (bind _returnvalue (Game|SpawnActorfromClass "/Game/Blueprints/LTTL2/LTTL_Train_BP_2.LTTL_Train_BP_2_C" (Math|Transform|MakeTransform "0, 0, 0" "0, 0, 0" "1,1,1") "Undefined" 0 0))
    (Utilities|Array|Add (Variables|Default|GetTrains) _returnvalue)
    (Class|VehicleTrain|StartTrain _returnvalue (Variables|Default|GetTrack) (* _index (/ (Spline|GetSplineLength (Variables|/Script/FP82MasterNew.TrackBase|GetSpline (Variables|Default|GetTrack))) (Math|Conversions|ToFloat(Integer) (Variables|Default|GetTrainsAmount)))) 5.5e+02))
  (Variables|Default|SetComplete? true))

(event EventTick
  (params (DeltaSeconds :type Float%20%28single-precision%29))
  (bind _returnvalue (Game|GetPlayerController 0))
  (bind _returnvalue_2 (Pawn|GetControlRotation _returnvalue :!class /Script/Engine.Controller))
  (if (Variables|Default|GetComplete?)
    (if (Variables|Default|GetCharacterRiding)
      (bind _output_get (Variables|Default|SetCurrentControlRotation (Math|Rotator|MakeRotator (* (- (.roll (Variables|Default|GetOriginalControlRotation)) (.roll _returnvalue_2)) -1.0) (* (- (.pitch (Variables|Default|GetOriginalControlRotation)) (.pitch _returnvalue_2)) -1.0) (* (- (.yaw (Variables|Default|GetOriginalControlRotation)) (.yaw _returnvalue_2)) -1.0))))
      (Transformation|SetRelativeRotation (Variables|Default|GetWedwayCam) _output_get false false)
      (else
        (for (_array_element _array_index) (Variables|Default|GetTrains)
          (bind _returnvalue_3 (Actor|GetActorOfClass "/Game/Blueprints/LttL/LTTL_Overlap.LTTL_Overlap_C"))
          (if (Collision|IsOverlappingActor _returnvalue_3 (Utilities|Array|Get(acopy) (Variables|/Script/FP82MasterNew.VehicleTrain|GetRideVehicles _array_element)) :!class /Script/Engine.Actor)
            (Variables|Default|SetTrainNum _array_index)
            (for (_array_element_2 _array_index_2) (Variables|/Script/FP82MasterNew.VehicleTrain|GetRideVehicles _array_element)
              (if (Collision|IsOverlappingActor (Game|GetPlayerCharacter 0) _array_element_2 :!class /Script/Engine.Actor)
                (Variables|Default|SetCarNum _array_index_2)
                (Variables|Default|SetOriginalControlRotation (Pawn|GetControlRotation (Game|GetPlayerController 0) :!class /Script/Engine.Controller))
                (Variables|Default|SetCurrentControlRotation (Math|Rotator|MakeRotator 0.0 0.0 0.0))
                (bind _returnvalue_4 (UserInterface|CreateWidget "/Game/Assets/Widgets/Info_Widget.Info_Widget_C" 0 "Press L to Ride"))
                (UserInterface|Viewport|AddtoViewport _returnvalue_4 0)))))))))

(event Input|ActionEvents|InputActionInteract
  (params (Key :type Key%20Structure :default "None")))

(fn ConstructionScript)

(fn ToggleWedwayView
  (params (TrainNum :type Integer) (CarNum :type Integer) (TransitionTime :type Float%20%28single-precision%29) (OrigSitting :type Boolean))
  (bind _returnvalue (Game|GetPlayerController 0))
  (bind _foundwidgets (Widget|GetAllWidgetsOfClass "/Game/Assets/Widgets/Info_Widget.Info_Widget_C" true))
  (Widget|RemovefromParent _foundwidgets)
  (Utilities|FlowControl|Sequence
    (:then_0
      (bind _asdefault_character (Utilities|Casting|CastToDefaultCharacter (Game|Player|GetPlayerPawn 0)))
      (Variables|Default|SetDefaultCharacterRef _asdefault_character))
    (:then_1
      (if (Variables|Default|GetCharacterRiding)
        (Pawn|SetControlRotation (Game|GetPlayerController 0) (Variables|Default|GetOriginalControlRotation))
        (Transformation|Teleport (Game|GetPlayerCharacter 0) "-24600.000000,220.000000,125.000000" "0.000000,90.000000,0.000000")
        (Game|Player|SetViewTargetwithBlend (Game|GetPlayerController 0) (Game|Player|GetPlayerPawn 0) TransitionTime "VTBlend_Linear" 0.0 false)
        (Variables|Default|SetCharacterRiding false)
        (Input|DisableInput (Game|GetPlayerController 0))
        (Viewport|RemoveAllWidgets)
        (else
          (bind _aslttlcar_bp (Utilities|Casting|CastToLTTLCar_BP (Utilities|Array|Get(acopy) (Variables|/Script/FP82MasterNew.VehicleTrain|GetRideVehicles (Utilities|Array|Get(acopy) (Variables|Default|GetTrains) TrainNum)) CarNum)))
          (Transformation|AttachComponentToComponent self (Variables|/Game/Blueprints/LttL/LTTLCar_BP.LTTLCar_BP_C|GetSittingPosition _aslttlcar_bp) "None" "SnapToTarget" "SnapToTarget" "KeepRelative" true)
          (Game|Player|SetViewTargetwithBlend _returnvalue self TransitionTime "VTBlend_Linear" 0.0 false)
          (Variables|Default|SetOriginalControlRotation (Pawn|GetControlRotation _returnvalue :!class /Script/Engine.Controller))
          (Variables|Default|SetCharacterRiding true)
          (Input|EnableInput (Game|GetPlayerController 0)))))))