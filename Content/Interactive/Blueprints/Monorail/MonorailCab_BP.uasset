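; MonorailCab_BP is a monorail cab with animated doors, a changeable color material and adjustable audio volume.
; DoorOperation plays a timeline forward to open or in reverse to close, swinging doors through 180 degrees of yaw.
; The FlippedDoors flag selects between standard and mirrored door sets, with the mirrored set rotating inversely.
; Other events apply a material to the body and doors and set the audio volume multiplier.
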(event Custom|SetMonorailColorMat
  (params (Material :type Material%20Interface%20Object%20Reference))
  (Rendering|Material|SetMaterial (Variables|Default|GetStaticMesh) 1 Material))

(event Custom|DoorOperation
  (params (Open :type Boolean))
  (if Open
    (bind _doorvalue (Timeline|Timeline_0 PlayFromStart)
      (:Update
        (if (Variables|Default|GetFlippedDoors)
          (Transformation|SetRelativeRotation (Variables|Default|GetDoor2) (Math|Rotator|MakeRotator 0.0 0.0 (* _doorvalue 1.8e+02)) false false)
          (else
            (Transformation|SetRelativeRotation (Variables|Default|GetDoorFlipped2) (Math|Rotator|MakeRotator 0.0 0.0 (- 1.8e+02 (* _doorvalue 1.8e+02))) false false)))))
    (else
      (Timeline|Timeline_0 ReverseFromEnd))))

(event Custom|ChangeVolume
  (params (NewVolume :type Float%20%28double-precision%29))
  (Audio|Components|Audio|SetVolumeMultiplier (Variables|Default|GetAudio) NewVolume :!class /Script/Engine.AudioComponent))

(fn ConstructionScript)