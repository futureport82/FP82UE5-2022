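; Monorail train actor that spawns and controls its cars, handling speed, doors and shared color material.
; BeginPlay builds the car list, typing cars by index and inserting spacers after the first four.
; Speed changes ease through a timeline, while a trigger-driven stop routine times halting, doors and departure.
; During stops it can switch a riding character to first person via the train handler, depending on camera location.
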(event Custom|SetMonorailColorMat
  (params (Material :type Material%20Interface%20Object%20Reference))
  (for _array_element (Variables|Default|GetRideVehicles)
    (bind _asmonorail_car_interactive_bp (Utilities|Casting|CastToMonorailCar_Interactive_BP _array_element))
    (Default|SetMonorailColorMat _asmonorail_car_interactive_bp Material)))

(event Custom|ChangeSpeed
  (params (SpeedType :type ETrainMode%20Enum :default "None") (SpeedScalar :type Float%20%28double-precision%29) (TrackTrigger :type Track%20Trigger%20Object%20Reference))
  (if (Utilities|Enum|NotEqual(Enum) (Variables|Default|GetCurrentMode) "None")
    (Utilities|FlowControl|Sequence
      (:then_0
        (Variables|Default|SetStartSpeed (Variables|Default|GetCurrentSpeed)))
      (:then_1
        (bind _output_get (Variables|Default|SetCurrentMode SpeedType))
        (switch Utilities|FlowControl|Switch|SwitchonETrainMode _output_get
          (:Idle
            (Variables|Default|SetTargetSpeed 0.0))
          (:Travel
            (Variables|Default|SetTargetSpeed SpeedScalar))
          (:Loading
            (Variables|Default|SetTargetSpeed (Variables|Default|GetMinSpeed)))
          (:SpeedScalar
            (Variables|Default|SetTargetSpeed (* (Variables|Default|GetMaxSpeed) SpeedScalar)))))
      (:then_2
        (bind _newtrack_0 (Timeline|Timeline_0 PlayFromStart)
          (:Update
            (Variables|Default|SetCurrentSpeed (Math|Float|Lerp (Variables|Default|GetStartSpeed) (Variables|Default|GetTargetSpeed) _newtrack_0))))))))

(event Custom|ChangeRandomMaterial
  (Utilities|FlowControl|DoOnce false :!label _label
    (:Completed
      (Utilities|FlowControl|Sequence
        (:then_0
          (bind _output (Default|RandomMonorailMaterial (Variables|Default|GetMonorailHandler)))
          (CallFunction|SetMonorailColorMat _output))
        (:then_1
          (Utilities|FlowControl|Delay 5.0)
          (goto _label Reset))))))

(event Custom|StartStopRoutine
  (params (Trigger :type Track%20Trigger%20Object%20Reference))
  (if (!= (Variables|Default|GetLastTrigger) Trigger)
    (Variables|Default|SetLastTrigger Trigger)
    (if (Utilities|Enum|NotEqual(Enum) (Variables|Default|GetCurrentMode) "Stop")
      (Variables|Default|SetCurrentMode "Stop")
      (CallFunction|ChangeSpeed "SpeedScalar" 0.0)
      (Utilities|FlowControl|Delay 3.0)
      (CallFunction|DoorOperation true)
      (bind _returnvalue (Actor|GetActorOfClass "/Game/Interactive/Blueprints/Monorail/MonorailTrainHandler_BP.MonorailTrainHandler_BP_C"))
      (Variables|Default|SetCharacterRiding? (Variables|/Game/Interactive/Blueprints/Monorail/MonorailTrainHandler_BP.MonorailTrainHandler_BP_C|GetCharacterRiding _returnvalue))
      (if (and (Variables|/Game/Interactive/Blueprints/Monorail/MonorailTrainHandler_BP.MonorailTrainHandler_BP_C|GetCharacterRiding _returnvalue) (and (< (.x (Transformation|GetWorldLocation (Variables|/Game/Interactive/Blueprints/Monorail/MonorailTrainHandler_BP.MonorailTrainHandler_BP_C|GetWedwayCam _returnvalue))) -1.6e+03) (< (.y (Transformation|GetWorldLocation (Variables|/Game/Interactive/Blueprints/Monorail/MonorailTrainHandler_BP.MonorailTrainHandler_BP_C|GetWedwayCam _returnvalue))) -2.9e+04)))
        (Utilities|FlowControl|Delay 2.0)
        (Default|SwitchtoFirstPerson _returnvalue 5.0))
      (Utilities|FlowControl|Delay 3e+01)
      (CallFunction|DoorOperation false)
      (Utilities|FlowControl|Delay 4.0)
      (CallFunction|ChangeSpeed "SpeedScalar" 0.15 Trigger)
      (Utilities|FlowControl|Delay 15.0)
      (Variables|Default|SetCurrentMode "Travel")
      (Variables|Default|SetLastTrigger 0))))

(event Custom|DoorOperation
  (params (Open :type Boolean))
  (for _array_element (Variables|Default|GetRideVehicles)
    (bind _asmonorail_car_interactive_bp (Utilities|Casting|CastToMonorailCar_Interactive_BP _array_element))
    (Default|DoorOperation _asmonorail_car_interactive_bp Open)))

(event EventBeginPlay
  (Utilities|FlowControl|Sequence
    (:then_0
      (Utilities|Array|Clear (Variables|Default|GetRideVehicles)))
    (:then_2
      (for _index (range 0 (- (Variables|Default|GetCarAmount) 1))
        (bind _returnvalue (Game|SpawnActorfromClass "/Game/Interactive/Blueprints/Monorail/MonorailCar_Interactive_BP.MonorailCar_Interactive_BP_C" (Math|Transform|MakeTransform "0, 0, 0" "0, 0, 0" "1.000000,1.000000,1.000000") "Undefined" 0 0))
        (Utilities|FlowControl|Sequence
          (:then_0
            (Variables|/Script/MainUE5Scratch.RideVehicle|SetSmoothRotation _returnvalue true)
            (Variables|/Script/MainUE5Scratch.RideVehicle|SetSmoothRotationAmt _returnvalue 1e+01))
          (:then_1
            (Variables|/Game/Interactive/Blueprints/Monorail/MonorailCar_Interactive_BP.MonorailCar_Interactive_BP_C|SetVehicleTrain _returnvalue self))
          (:then_2
            (Utilities|Array|Add (Variables|Default|GetRideVehicles) _returnvalue))
          (:then_3
            (switch int _index
              (:0
                (Default|AssignMonorailCarType _returnvalue "NewEnumerator0")
                ;[1 1 1] Add Spacer
                (bind _returnvalue_2 (Game|SpawnActorfromClass "/Game/Interactive/Blueprints/Monorail/MonorailCar_Interactive_BP.MonorailCar_Interactive_BP_C" (Math|Transform|MakeTransform "0, 0, 0" "0, 0, 0" "1.000000,1.000000,1.000000") "Undefined" 0 0 :!label _label))
                (Utilities|FlowControl|Sequence
                  (:then_0
                    (Variables|/Script/MainUE5Scratch.RideVehicle|SetSmoothRotation _returnvalue_2 true)
                    (Variables|/Script/MainUE5Scratch.RideVehicle|SetSmoothRotationAmt _returnvalue_2 1e+01))
                  (:then_1
                    (Variables|/Game/Interactive/Blueprints/Monorail/MonorailCar_Interactive_BP.MonorailCar_Interactive_BP_C|SetVehicleTrain _returnvalue_2 self))
                  (:then_2
                    (Utilities|Array|Add (Variables|Default|GetRideVehicles) _returnvalue_2))
                  (:then_3
                    (Default|AssignMonorailCarType _returnvalue_2 "NewEnumerator3"))))
              (:1
                (Default|AssignMonorailCarType _returnvalue "NewEnumerator1" :!label _label_2)
                (goto _label))
              (:2
                (goto _label_2))
              (:3
                (goto _label_2))
              (:4
                (Default|AssignMonorailCarType _returnvalue "NewEnumerator2")))))))))

(event Input|ActionEvents|InputActionInteract
  (params (Key :type Key%20Structure :default "None")))

(fn ConstructionScript)