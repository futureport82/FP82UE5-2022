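; Interactive monorail train car that reacts to TrackTrigger_BP volumes along the track.
; Overlaps drive VehicleTrain speed, stops and color changes, cab volume, narration, music, and FWE/FWW loading while riding.
; A car type selects the cab, mid-car or spacer child actor, which receives material and DoorOperation calls.
; The trigger-driven door timeline has an empty update, so it moves nothing.
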(event OnComponentBeginOverlap(TriggerCollision)
  (params (OverlappedComponent :type Primitive%20Component%20Object%20Reference) (OtherActor :type Actor%20Object%20Reference) (OtherComp :type Primitive%20Component%20Object%20Reference) (OtherBodyIndex :type Integer) (bFromSweep :type Boolean) (SweepResult :type Hit%20Result%20Structure%20%28by%20ref%29))
  (bind _returnvalue (Game|GetGameInstance))
  (bind _vehicletrain (Variables|Default|GetVehicleTrain))
  (bind _narration (Variables|Default|GetNarration))
  (bind _bgm (Variables|Default|GetBGM))
  (bind _astrack_trigger_bp (Utilities|Casting|CastToTrackTrigger_BP OtherActor))
  (Utilities|FlowControl|Sequence
    (:then_0
      (switch Utilities|FlowControl|Switch|SwitchonETrainMode "None"
        (:None
          (switch Utilities|FlowControl|Switch|SwitchonETrackTrigger (Variables|/Game/Interactive/Blueprints/Monorail/TrackTrigger_BP.TrackTrigger_BP_C|GetTrackEvent _astrack_trigger_bp)
            (:Narration
              (Audio|Components|Audio|SetSound _narration (Variables|/Game/Interactive/Blueprints/Monorail/TrackTrigger_BP.TrackTrigger_BP_C|GetWEDWAYNarration _astrack_trigger_bp))
              (Audio|Components|Audio|Play (Variables|Default|GetNarration) 0.0))
            (:StopNarration
              (Audio|Components|Audio|FadeOut _narration 1.5 0.0 "Linear" :!class /Script/Engine.AudioComponent))
            (:StartBGM
              (Audio|Components|Audio|SetSound _bgm (Variables|/Game/Interactive/Blueprints/Monorail/TrackTrigger_BP.TrackTrigger_BP_C|GetWEDWAYBGM _astrack_trigger_bp))
              (Audio|Components|Audio|SetVolumeMultiplier _bgm (Variables|/Game/Interactive/Blueprints/Monorail/TrackTrigger_BP.TrackTrigger_BP_C|GetWEDWAYBGMVolume _astrack_trigger_bp) :!class /Script/Engine.AudioComponent)
              (Audio|Components|Audio|FadeIn _bgm 1.5 (Variables|/Game/Interactive/Blueprints/Monorail/TrackTrigger_BP.TrackTrigger_BP_C|GetWEDWAYBGMVolume _astrack_trigger_bp) 0.0 "Linear" :!class /Script/Engine.AudioComponent)
              (Audio|Components|Audio|Play _bgm (Variables|/Game/Interactive/Blueprints/Monorail/TrackTrigger_BP.TrackTrigger_BP_C|GetWEDWAYBGMStart _astrack_trigger_bp)))
            (:LoadFWE
              (bind _asfp82game_instance (Utilities|Casting|CastToFP82GameInstance _returnvalue))
              (if (Variables|/Game/Assets/Blueprints/FP82GameInstance.FP82GameInstance_C|GetRiding%20Monorail _asfp82game_instance)
                (bind _returnvalue_2 (Actor|GetActorOfClass "/Game/FWE_Unload_FWW_Blueprint.FWE_Unload_FWW_Blueprint_C"))
                (Default|LoadFWEBase _returnvalue_2)))
            (:LoadFWW
              (bind _asfp82game_instance_2 (Utilities|Casting|CastToFP82GameInstance _returnvalue))
              (if (Variables|/Game/Assets/Blueprints/FP82GameInstance.FP82GameInstance_C|GetRiding%20Monorail _asfp82game_instance_2)
                (bind _returnvalue_3 (Actor|GetActorOfClass "/Game/FWW_Unload_FWE_Blueprint.FWW_Unload_FWE_Blueprint_C"))
                (Default|LoadFWWBase _returnvalue_3)))))
        (:Idle
          (Default|ChangeSpeed _vehicletrain (Variables|/Game/Interactive/Blueprints/Monorail/TrackTrigger_BP.TrackTrigger_BP_C|GetTrainMode _astrack_trigger_bp) (Variables|/Game/Interactive/Blueprints/Monorail/TrackTrigger_BP.TrackTrigger_BP_C|GetSpeedScalar _astrack_trigger_bp) _astrack_trigger_bp :!label _label)
          (bind _asmonorail_cab_bp (Utilities|Casting|CastToMonorailCab_BP (Variables|/Script/Engine.ChildActorComponent|GetChildActor (Variables|Default|GetMonorailCar))))
          (Default|ChangeVolume _asmonorail_cab_bp (* (Math|Vector|VectorLength (Transformation|GetVelocity _vehicletrain)) 0.6)))
        (:Travel
          (goto _label))
        (:Loading
          (goto _label))
        (:DoorOpen
          (CallFunction|DoorFunctionality true))
        (:DoorClose
          (CallFunction|DoorFunctionality false))
        (:SpeedScalar
          (goto _label))
        (:Stop
          (Default|StartStopRoutine (Variables|Default|GetVehicleTrain) _astrack_trigger_bp))))
    (:then_1
      (switch Utilities|FlowControl|Switch|SwitchonETrackTrigger (Variables|/Game/Interactive/Blueprints/Monorail/TrackTrigger_BP.TrackTrigger_BP_C|GetTrackEvent _astrack_trigger_bp)
        (:ChangeColor
          (Default|ChangeRandomMaterial (Variables|Default|GetVehicleTrain)))))))

(event Custom|SetMonorailColorMat
  (params (Material :type Material%20Interface%20Object%20Reference))
  (bind _monorailcar (Variables|Default|GetMonorailCar))
  (bind _childactor (Variables|/Script/Engine.ChildActorComponent|GetChildActor _monorailcar))
  (bind _asmonorail_cab_bp (Utilities|Casting|CastToMonorailCab_BP _childactor)
    (:then
      (Default|SetMonorailColorMat _asmonorail_cab_bp Material))
    (:CastFailed
      (bind _asmonorail_car_bp (Utilities|Casting|CastToMonorailCar_BP _childactor))
      (Default|SetMonorailColorMat _asmonorail_car_bp Material))))

(event Custom|DoorOperation
  (params (Open :type Boolean))
  (bind _asmonorail_cab_bp (Utilities|Casting|CastToMonorailCab_BP (Variables|/Script/Engine.ChildActorComponent|GetChildActor (Variables|Default|GetMonorailCar)))
    (:then
      (Default|DoorOperation _asmonorail_cab_bp Open))
    (:CastFailed
      (bind _asmonorail_car_bp (Utilities|Casting|CastToMonorailCar_BP (Variables|/Script/Engine.ChildActorComponent|GetChildActor (Variables|Default|GetMonorailCar))))
      (Default|DoorOperation _asmonorail_car_bp Open))))

(event Custom|AssignMonorailCarType
  (params (CarType :type MonorailCarType%20Enum :default "NewEnumerator0"))
  (switch Utilities|FlowControl|Switch|SwitchonMonorailCarType CarType
    (:NewEnumerator0
      (ChildActorComponent|SetChildActorClass (Variables|Default|GetMonorailCar) "/Game/Interactive/Blueprints/Monorail/MonorailCab_BP.MonorailCab_BP_C")
      (Transformation|SetRelativeRotation (Variables|Default|GetMonorailCar) "0,-180.000000, 0" false false))
    (:NewEnumerator1
      (ChildActorComponent|SetChildActorClass (Variables|Default|GetMonorailCar) "/Game/Interactive/Blueprints/Monorail/MonorailCar_BP.MonorailCar_BP_C"))
    (:NewEnumerator2
      (ChildActorComponent|SetChildActorClass (Variables|Default|GetMonorailCar) "/Game/Interactive/Blueprints/Monorail/MonorailCab_BP.MonorailCab_BP_C")
      (Transformation|SetRelativeRotation (Variables|Default|GetMonorailCar) "0, 0, 0" false false)
      (bind _asmonorail_cab_bp (Utilities|Casting|CastToMonorailCab_BP (Variables|/Script/Engine.ChildActorComponent|GetChildActor (Variables|Default|GetMonorailCar))))
      (Variables|/Game/Interactive/Blueprints/Monorail/MonorailCab_BP.MonorailCab_BP_C|SetFlippedDoors _asmonorail_cab_bp true))
    (:NewEnumerator3
      (ChildActorComponent|SetChildActorClass (Variables|Default|GetMonorailCar) "/Game/Interactive/Blueprints/Monorail/MonorailSpacer_BP.MonorailSpacer_BP_C"))))

(event Custom|DoorFunctionality
  (params (Open :type Boolean))
  (if Open
    (bind _newtrack_0 (Timeline|DoorOpenClose PlayFromStart)
      (:Update
        (Utilities|FlowControl|Sequence)))
    (else
      (Timeline|DoorOpenClose ReverseFromEnd))))

(event EventTick
  (params (DeltaSeconds :type Float%20%28single-precision%29)))

(fn ConstructionScript)