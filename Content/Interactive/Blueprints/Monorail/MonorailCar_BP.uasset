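; MonorailCar_BP is a monorail car actor with operable doors, a changeable color material and a running sound.
; DoorOperation plays or reverses the OpenRoutine timeline, which drives the yaw of only the four flipped door meshes.
; SetMonorailColorMat applies a material to slot 1 of the body and all eight doors, and ChangeVolume scales the Running audio.
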(event Custom|SetMonorailColorMat
  (params (Material :type Material%20Interface%20Object%20Reference))
  (Rendering|Material|SetMaterial (Variables|Default|GetStaticMesh) 1 Material))

(event Custom|DoorOperation
  (params (Open :type Boolean))
  (if Open
    (bind _doorvalue (Timeline|OpenRoutine PlayFromStart)
      (:Update
        (Transformation|SetRelativeRotation (Variables|Default|GetDoorFlipped2) (Math|Rotator|MakeRotator 0.0 0.0 (- 1.8e+02 (* _doorvalue 1.8e+02))) false false)))
    (else
      (Timeline|OpenRoutine ReverseFromEnd))))

(event Custom|ChangeVolume
  (params (NewVolume :type Float%20%28double-precision%29))
  (Audio|Components|Audio|SetVolumeMultiplier (Variables|Default|GetRunning) NewVolume :!class /Script/Engine.AudioComponent))

(event EventBeginPlay)

(event Collision|EventActorBeginOverlap
  (params (OtherActor :type Actor%20Object%20Reference)))

(event EventTick
  (params (DeltaSeconds :type Float%20%28single-precision%29)))

(fn ConstructionScript)