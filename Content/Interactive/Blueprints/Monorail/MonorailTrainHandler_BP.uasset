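; Monorail handler that spawns evenly spaced trains along a track and runs the player's first-load ride aboard one.
; Each train gets a random color material, drawn without repeats until the pool refills.
; Riding attaches the view to a car of the first train, with control rotation deltas driving the camera.
; Interact skips the ride, loading the PostMonorail level, teleporting the character and restoring the pawn view.
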(event Custom|SwitchToFirstPerson
  (params (BlendTime :type Float%20%28double-precision%29))
  (Game|LoadStreamLevel(byName) "PostMonorail" true)
  (CallFunction|ToggleMonorailView BlendTime))

(event EventBeginPlay
  (Utilities|FlowControl|Sequence
    (:then_0
      (for _index (range 0 (- (Variables|Default|GetTrainsAmount) 1))
        (bind _returnvalue (Game|SpawnActorfromClass "/Game/Interactive/Blueprints/Monorail/MonorailTrain_BP.MonorailTrain_BP_C" (Math|Transform|MakeTransform "0, 0, 0" "0, 0, 0" "1.000000,1.000000,1.000000") "Undefined" 0 0))
        (Utilities|Array|Add (Variables|Default|GetTrains) _returnvalue)
        (Variables|/Game/Interactive/Blueprints/Monorail/MonorailTrain_BP.MonorailTrain_BP_C|SetMonorailHandler _returnvalue self)
        (bind _output (CallFunction|RandomMonorailMaterial))
        (Default|SetMonorailColorMat _returnvalue _output)
        (Class|VehicleTrain|StartTrain _returnvalue (Variables|Default|GetTrack) (* _index (/ (Spline|GetSplineLength (Variables|/Script/MainUE5Scratch.TrackBase|GetSpline (Variables|Default|GetTrack))) (Math|Conversions|ToFloat(Integer) (Variables|Default|GetTrainsAmount)))) 1.05e+03)
        (Default|ChangeSpeed _returnvalue "SpeedScalar" 0.4)))
    (:then_1
      ;[1 1 1] Enables Riding Monorail
      (bind _asfp82game_instance (Utilities|Casting|CastToFP82GameInstance (Game|GetGameInstance)))
      (if (Variables|/Game/Assets/Blueprints/FP82GameInstance.FP82GameInstance_C|GetFirstLoad? _asfp82game_instance)
        (CallFunction|ToggleMonorailView 0.0)
        (Utilities|FlowControl|Delay 15.0)
        (bind _returnvalue_2 (UserInterface|CreateWidget "/Game/Assets/Widgets/Info_Widget.Info_Widget_C" 0 "Press Space Bar to Skip"))
        (Default|Fadein _returnvalue_2)
        (UserInterface|Viewport|AddtoViewport _returnvalue_2 0)
        (Input|EnableInput (Game|GetPlayerController 0))
        (Utilities|FlowControl|Delay 5.0)
        (Widget|RemovefromParent _returnvalue_2)))))

(event EventTick
  (params (DeltaSeconds :type Float%20%28single-precision%29))
  (bind _returnvalue (Game|GetPlayerController 0))
  (bind _originalcontrolrotation (Variables|Default|GetOriginalControlRotation))
  (bind _returnvalue_2 (Pawn|GetControlRotation _returnvalue :!class /Script/Engine.Controller))
  (if (Variables|Default|GetCharacterRiding)
    (bind _output_get (Variables|Default|SetCurrentControlRotation (Math|Rotator|MakeRotator (* (- (.roll _originalcontrolrotation) (.roll _returnvalue_2)) -1.0) (* (- (.pitch _originalcontrolrotation) (.pitch _returnvalue_2)) -1.0) (* (- (.yaw _originalcontrolrotation) (.yaw _returnvalue_2)) -1.0))))
    (Transformation|SetRelativeRotation (Variables|Default|GetWedwayCam) _output_get false false)))

(event Input|ActionEvents|InputActionInteract
  (params (Key :type Key%20Structure :default "None"))
  (:Pressed
    (if (Variables|Default|GetCharacterRiding)
      (Viewport|RemoveAllWidgets)
      (bind _returnvalue (UserInterface|CreateWidget "/Game/Assets/Widgets/LevelFadeUp_Pavilion.LevelFadeUp_Pavilion_C"))
      (UserInterface|Viewport|AddtoViewport _returnvalue 0)
      (CallFunction|SwitchtoFirstPerson 0.0)
      (Input|DisableInput (Game|GetPlayerController 0)))))

(fn ConstructionScript)

(fn ToggleMonorailView
  (params (BlendTime :type Float%20%28double-precision%29))
  (bind _returnvalue (Game|GetPlayerController 0))
  (Utilities|FlowControl|Sequence
    (:then_0
      (bind _asdefault_character (Utilities|Casting|CastToDefaultCharacter (Game|Player|GetPlayerPawn 0)))
      (Variables|Default|SetDefaultCharacterRef _asdefault_character))
    (:then_1
      (if (Variables|Default|GetCharacterRiding)
        (Pawn|SetControlRotation (Game|GetPlayerController 0) (Variables|Default|GetOriginalControlRotation))
        (Transformation|Teleport (Game|GetPlayerCharacter 0) "-1808.000000,-30580.000000,550.000000" "0, 0, 0")
        (Game|Player|SetViewTargetwithBlend (Game|GetPlayerController 0) (Game|Player|GetPlayerPawn 0) BlendTime "VTBlend_Linear" 0.0 false)
        (Variables|Default|SetCharacterRiding false)
        (bind _asfp82game_instance (Utilities|Casting|CastToFP82GameInstance (Game|GetGameInstance)))
        (Variables|/Game/Assets/Blueprints/FP82GameInstance.FP82GameInstance_C|SetRiding%20Monorail _asfp82game_instance false)
        (else
          (bind _asmonorail_car_interactive_bp (Utilities|Casting|CastToMonorailCar_Interactive_BP (Utilities|Array|Get(acopy) (Variables|/Script/MainUE5Scratch.VehicleTrain|GetRideVehicles (Utilities|Array|Get(acopy) (Variables|Default|GetTrains))) 2)))
          (Transformation|AttachComponentToComponent self (Variables|/Game/Interactive/Blueprints/Monorail/MonorailCar_Interactive_BP.MonorailCar_Interactive_BP_C|GetSittingPosition _asmonorail_car_interactive_bp) "None" "SnapToTarget" "SnapToTarget" "KeepRelative" true)
          (Game|Player|SetViewTargetwithBlend _returnvalue self 0.0 "VTBlend_Linear" 0.0 false)
          (Variables|Default|SetCharacterRiding true)
          (Variables|Default|SetOriginalControlRotation (Pawn|GetControlRotation _returnvalue :!class /Script/Engine.Controller))
          (bind _asfp82game_instance_2 (Utilities|Casting|CastToFP82GameInstance (Game|GetGameInstance)))
          (Variables|/Game/Assets/Blueprints/FP82GameInstance.FP82GameInstance_C|SetRiding%20Monorail _asfp82game_instance_2 true))))))

(fn RandomMonorailMaterial
  (Utilities|FlowControl|Sequence
    (:then_0
      ;[1 1 1] Refills materials once used up
      (if (<= (Utilities|Array|Length (Variables|Default|GetMonorailColorMaterials)) 0)
        (Variables|Default|SetMonorailColorMaterials (Variables|Default|GetMonorailColorMaterials__ORIGINAL))))
    (:then_1
      (LocalVariables|SetRandomI (Math|Random|RandomIntegerinRange 0 (- (Utilities|Array|Length (Variables|Default|GetMonorailColorMaterials)) 1)))
      (LocalVariables|SetMaterialOut (Utilities|Array|Get(acopy) (Variables|Default|GetMonorailColorMaterials) (LocalVariables|GetRandomI))))
    (:then_2
      (Utilities|Array|RemoveIndex (Variables|Default|GetMonorailColorMaterials) (LocalVariables|GetRandomI)))
    (:then_3
      (return (LocalVariables|GetMaterialOut)))))