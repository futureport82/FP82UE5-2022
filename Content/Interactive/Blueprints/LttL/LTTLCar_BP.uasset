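; LTTLCar_BP is a ride vehicle car that responds to track trigger volumes as it moves.
; On overlap with a TrackTrigger_BP, its track event plays or fades narration and background music using sounds and settings from the trigger.
; The same overlap then passes the trigger's train mode and speed scalar to VehicleTrain to change speed.
; Leftover FWW/FWE area-loading logic for WEDWAY and Monorail riders is never executed.
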(event OnComponentBeginOverlap(TriggerCollision)
  (params (OverlappedComponent :type Primitive%20Component%20Object%20Reference) (OtherActor :type Actor%20Object%20Reference) (OtherComp :type Primitive%20Component%20Object%20Reference) (OtherBodyIndex :type Integer) (bFromSweep :type Boolean) (SweepResult :type Hit%20Result%20Structure%20%28by%20ref%29))
  (bind _narrationbgm (Variables|Default|GetNarrationBGM))
  (bind _narrationbgm_2 (Variables|Default|GetNarrationBGM))
  (bind _narrationbgm_3 (Variables|Default|GetNarrationBGM))
  (bind _astrack_trigger_bp (Utilities|Casting|CastToTrackTrigger_BP OtherActor))
  (Utilities|FlowControl|Sequence
    (:then_0
      (switch Utilities|FlowControl|Switch|SwitchonETrackTrigger (Variables|/Game/Blueprints/TrackTrigger_BP.TrackTrigger_BP_C|GetTrackEvent _astrack_trigger_bp)
        (:Narration
          (Audio|Components|Audio|SetSound (Variables|Default|GetNarrationAudio) (Variables|/Game/Blueprints/TrackTrigger_BP.TrackTrigger_BP_C|GetWEDWAYNarration _astrack_trigger_bp))
          (Audio|Components|Audio|FadeOut _narrationbgm 1.0 0.0 "Linear" :!class /Script/Engine.AudioComponent)
          (Audio|Components|Audio|SetSound _narrationbgm (Variables|/Game/Blueprints/TrackTrigger_BP.TrackTrigger_BP_C|GetWEDWAYBGM _astrack_trigger_bp))
          (Audio|Components|Audio|Play (Variables|Default|GetNarrationAudio) 0.0)
          (Audio|Components|Audio|SetVolumeMultiplier _narrationbgm_2 (Variables|/Game/Blueprints/TrackTrigger_BP.TrackTrigger_BP_C|GetWEDWAYBGMVolume _astrack_trigger_bp) :!class /Script/Engine.AudioComponent)
          (Audio|Components|Audio|FadeIn _narrationbgm_2 0.5 (Variables|/Game/Blueprints/TrackTrigger_BP.TrackTrigger_BP_C|GetWEDWAYBGMVolume _astrack_trigger_bp) 0.0 "Linear" :!class /Script/Engine.AudioComponent)
          (Audio|Components|Audio|Play (Variables|Default|GetNarrationBGM) (Variables|/Game/Blueprints/TrackTrigger_BP.TrackTrigger_BP_C|GetWEDWAYBGMStart _astrack_trigger_bp)))
        (:StopNarration
          (Audio|Components|Audio|FadeOut (Variables|Default|GetNarrationAudio) 1.5 0.0 "Linear" :!class /Script/Engine.AudioComponent))
        (:StartBGM
          (Audio|Components|Audio|SetSound _narrationbgm_3 (Variables|/Game/Blueprints/TrackTrigger_BP.TrackTrigger_BP_C|GetWEDWAYBGM _astrack_trigger_bp))
          (Audio|Components|Audio|FadeIn _narrationbgm_3 1.5 (Variables|/Game/Blueprints/TrackTrigger_BP.TrackTrigger_BP_C|GetWEDWAYBGMVolume _astrack_trigger_bp) 0.0 "Linear" :!class /Script/Engine.AudioComponent)
          (Audio|Components|Audio|Play _narrationbgm_3 (Variables|/Game/Blueprints/TrackTrigger_BP.TrackTrigger_BP_C|GetWEDWAYBGMStart _astrack_trigger_bp)))
        (:EndBGM
          (Audio|Components|Audio|FadeOut _narrationbgm_3 2.0 0.0 "Linear" :!class /Script/Engine.AudioComponent))))
    (:then_1
      (switch Utilities|FlowControl|Switch|SwitchonETrainMode (Variables|/Game/Blueprints/TrackTrigger_BP.TrackTrigger_BP_C|GetTrainMode _astrack_trigger_bp)
        (:None
          _)
        (:Idle
          _)
        (:Travel
          _)
        (:Loading
          _))
      (Default|ChangeSpeed (Variables|Default|GetVehicleTrain) (Variables|/Game/Blueprints/TrackTrigger_BP.TrackTrigger_BP_C|GetTrainMode _astrack_trigger_bp) (Variables|/Game/Blueprints/TrackTrigger_BP.TrackTrigger_BP_C|GetSpeedScalar _astrack_trigger_bp)))))

(fn ConstructionScript)