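; JII_Entrance_Overlap is an overlap actor that serves as the entrance prompt for the JII ride.
; When a DefaultCharacter overlaps it, it shows an Info_Widget ride prompt and enables input from player controller 0.
; Pressing Interact clears all widgets and opens the JII_Ride_Entrance_Player widget.
; Leaving the overlap also clears all widgets but does not disable the actor's input.
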(event Collision|EventActorEndOverlap
  (params (OtherActor :type Actor%20Object%20Reference))
  (Utilities|Casting|CastToDefaultCharacter OtherActor)
  (Viewport|RemoveAllWidgets))

(event Collision|EventActorBeginOverlap
  (params (OtherActor :type Actor%20Object%20Reference))
  (Utilities|Casting|CastToDefaultCharacter OtherActor)
  (bind _returnvalue (UserInterface|CreateWidget "/Game/Assets/Widgets/Info_Widget.Info_Widget_C" 0 "Press Space to Ride"))
  (UserInterface|Viewport|AddtoViewport _returnvalue 0)
  (Input|EnableInput (Game|GetPlayerController 0)))

(event Input|ActionEvents|InputActionInteract
  (params (Key :type Key%20Structure :default "None"))
  (:Pressed
    (Viewport|RemoveAllWidgets)
    (bind _returnvalue (UserInterface|CreateWidget "/Game/Assets/Widgets/JII_Ride_Entrance_Player.JII_Ride_Entrance_Player_C"))
    (UserInterface|Viewport|AddtoViewport _returnvalue 0)))

(fn ConstructionScript)