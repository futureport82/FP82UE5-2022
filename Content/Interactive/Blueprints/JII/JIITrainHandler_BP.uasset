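; JII train handler that spawns evenly spaced trains along a track and manages the player's first-person WEDWAY ride.
; ToggleWedwayView either snaps to a car seat and blends the view to this actor, or teleports the player out, updating the game instance's riding flag.
; While riding, Tick turns control-rotation change into camera look.
; Events change train, car or seat via that toggle; entrance-overlap detection is present but never runs.
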(event Custom|SwitchToFirstPerson
  (params (TransitionTime :type Float%20%28single-precision%29))
  (CallFunction|ToggleWedwayView (Variables|Default|GetTrainNum) (Variables|Default|GetCarNum) TransitionTime true))

(event Custom|ChangeTrain
  (if (== (Variables|Default|GetTrainNum) 0)
    (Variables|Default|SetTrainNum (- (Variables|Default|GetTrainsAmount) 1))
    (else
      (Variables|Default|SetTrainNum (- (Variables|Default|GetTrainNum) 1))))
  (CallFunction|ToggleWedwayView (Variables|Default|GetTrainNum) (Variables|Default|GetCarNum) 0.0 (Variables|Default|GetOrig%20Sitting?))
  (Development|PrintString (Utilities|String|ToString(Integer) (Variables|Default|GetTrainNum))))

(event Custom|ChangeCar
  (if (== (Variables|Default|GetCarNum) 5)
    (Variables|Default|SetCarNum 0)
    (else
      (Variables|Default|SetCarNum (+ (Variables|Default|GetCarNum) 1))))
  (CallFunction|ToggleWedwayView (Variables|Default|GetTrainNum) (Variables|Default|GetCarNum) 0.0 (Variables|Default|GetOrig%20Sitting?)))

(event Custom|SwitchSitting
  (bind _trainnum (Variables|Default|GetTrainNum))
  (bind _carnum (Variables|Default|GetCarNum))
  (Utilities|FlowControl|FlipFlop
    (:A
      (CallFunction|ToggleWedwayView _trainnum _carnum 0.0 false)
      (Variables|Default|SetOrig%20Sitting? false))
    (:B
      (CallFunction|ToggleWedwayView _trainnum _carnum 0.0 true)
      (Variables|Default|SetOrig%20Sitting? true))))

(event EventBeginPlay
  (for _index (range 0 (- (Variables|Default|GetTrainsAmount) 1))
    (bind _returnvalue (Game|SpawnActorfromClass "/Game/Blueprints/JII/JIITrain_BP.JIITrain_BP_C" (Math|Transform|MakeTransform "0, 0, 0" "0, 0, 0" "1,1,1") "Undefined" 0 0))
    (Utilities|Array|Add (Variables|Default|GetTrains) _returnvalue)
    (Class|VehicleTrain|StartTrain _returnvalue (Variables|Default|GetTrack) (* _index (/ (Spline|GetSplineLength (Variables|/Script/FP82MasterNew.TrackBase|GetSpline (Variables|Default|GetTrack))) (Math|Conversions|ToFloat(Integer) (Variables|Default|GetTrainsAmount)))) 2.6e+02)))

(event EventTick
  (params (DeltaSeconds :type Float%20%28single-precision%29))
  (bind _returnvalue (Game|GetPlayerController 0))
  (bind _originalcontrolrotation (Variables|Default|GetOriginalControlRotation))
  (bind _returnvalue_2 (Pawn|GetControlRotation _returnvalue :!class /Script/Engine.Controller))
  (if (Variables|Default|GetCharacterRiding)
    (bind _output_get (Variables|Default|SetCurrentControlRotation (Math|Rotator|MakeRotator (* (- (.roll _originalcontrolrotation) (.roll _returnvalue_2)) -1.0) (* (- (.pitch _originalcontrolrotation) (.pitch _returnvalue_2)) -1.0) (* (- (.yaw _originalcontrolrotation) (.yaw _returnvalue_2)) -1.0))))
    (Transformation|SetRelativeRotation (Variables|Default|GetWedwayCam) _output_get false false)))

(event Input|ActionEvents|InputActionInteract
  (params (Key :type Key%20Structure :default "None"))
  (:Pressed
    (Utilities|FlowControl|FlipFlop
      (:A
        (bind _returnvalue (UserInterface|CreateWidget "/Game/Assets/Widgets/WEDWAYControls.WEDWAYControls_C"))
        (UserInterface|Viewport|AddtoViewport _returnvalue 0))
      (:B
        (bind _foundwidgets (Widget|GetAllWidgetsOfClass "/Game/Assets/Widgets/WEDWAYControls.WEDWAYControls_C" true))
        (Widget|RemovefromParent _foundwidgets)))))

(fn ConstructionScript)

(fn ToggleWedwayView
  (params (TrainNum :type Integer) (CarNum :type Integer) (TransitionTime :type Float%20%28single-precision%29) (OrigSitting :type Boolean))
  (bind _returnvalue (Game|GetPlayerController 0))
  (bind _foundwidgets (Widget|GetAllWidgetsOfClass "/Game/Assets/Widgets/Info_Widget.Info_Widget_C" true))
  (Widget|RemovefromParent _foundwidgets)
  (Utilities|FlowControl|Sequence
    (:then_0
      (bind _asdefault_character (Utilities|Casting|CastToDefaultCharacter (Game|Player|GetPlayerPawn 0)))
      (Variables|Default|SetDefaultCharacterRef _asdefault_character))
    (:then_1
      (if (Variables|Default|GetCharacterRiding)
        (Pawn|SetControlRotation (Game|GetPlayerController 0) (Variables|Default|GetOriginalControlRotation))
        (Transformation|Teleport (Game|GetPlayerCharacter 0) "-3225.000000,-15386.000000,450.000000" "0,90.000000, 0")
        (Game|Player|SetViewTargetwithBlend (Game|GetPlayerController 0) (Game|Player|GetPlayerPawn 0) TransitionTime "VTBlend_Linear" 0.0 false)
        (Variables|Default|SetCharacterRiding false)
        (Input|DisableInput (Game|GetPlayerController 0))
        (bind _asfp82game_instance (Utilities|Casting|CastToFP82GameInstance (Game|GetGameInstance)))
        (Variables|/Game/Assets/Blueprints/FP82GameInstance.FP82GameInstance_C|SetRiding%20WEDWAY _asfp82game_instance false)
        (else
          (bind _aswedway_car_bp (Utilities|Casting|CastToWedwayCar_BP (Utilities|Array|Get(acopy) (Variables|/Script/FP82MasterNew.VehicleTrain|GetRideVehicles (Utilities|Array|Get(acopy) (Variables|Default|GetTrains) TrainNum)) CarNum)))
          (if OrigSitting
            (Transformation|AttachComponentToComponent self (Variables|/Game/Blueprints/Wedway/WedwayCar_BP.WedwayCar_BP_C|GetSittingPosition _aswedway_car_bp) "None" "SnapToTarget" "SnapToTarget" "KeepRelative" true)
            (else
              (Transformation|AttachComponentToComponent self (Variables|/Game/Blueprints/Wedway/WedwayCar_BP.WedwayCar_BP_C|GetSittingPositionOpp _aswedway_car_bp) "None" "SnapToTarget" "SnapToTarget" "KeepRelative" true)))
          (Game|Player|SetViewTargetwithBlend _returnvalue self TransitionTime "VTBlend_Linear" 0.0 false)
          (Variables|Default|SetOriginalControlRotation (Pawn|GetControlRotation _returnvalue :!class /Script/Engine.Controller))
          (Variables|Default|SetCharacterRiding true)
          (bind _returnvalue_2 (UserInterface|CreateWidget "/Game/Assets/Widgets/Info_Widget.Info_Widget_C" 0 "Press Space Bar to View Controls"))
          (UserInterface|Viewport|AddtoViewport _returnvalue_2 0)
          (Default|Fade5 _returnvalue_2)
          (Input|EnableInput (Game|GetPlayerController 0))
          (bind _asfp82game_instance_2 (Utilities|Casting|CastToFP82GameInstance (Game|GetGameInstance)))
          (Variables|/Game/Assets/Blueprints/FP82GameInstance.FP82GameInstance_C|SetRiding%20WEDWAY _asfp82game_instance_2 true))))))