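; DefaultCharacter is a player character with axis-driven movement, mouse look and a hold-to-run action.
; Movement follows the actor's forward and right vectors, with forward input weighted more heavily, while look input is scaled by MouseSensitivity.
; Pressing or releasing Run switches CharacterMovement's max walk speed between run and walk values.
; A Relocate event moves the character to the LastLocation stored in FP82GameInstance.
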(event Custom|Relocate
  (bind _asfp82game_instance (Utilities|Casting|CastToFP82GameInstance (Game|GetGameInstance)))
  (Transformation|SetActorLocation (Variables|/Game/Assets/Blueprints/FP82GameInstance.FP82GameInstance_C|GetLastLocation _asfp82game_instance) false false))

(event EventBeginPlay
  (Variables|/Script/Engine.CharacterMovementComponent|SetMaxWalkSpeed (Variables|Character|GetCharacterMovement) 275.0))

(event Collision|EventActorBeginOverlap
  (params (OtherActor :type Actor%20Object%20Reference)))

(event Input|ActionEvents|InputActionRun
  (params (Key :type Key%20Structure :default "None"))
  (:Pressed
    (Variables|/Script/Engine.CharacterMovementComponent|SetMaxWalkSpeed (Variables|Character|GetCharacterMovement) 5e+02))
  (:Released
    (Variables|/Script/Engine.CharacterMovementComponent|SetMaxWalkSpeed (Variables|Character|GetCharacterMovement) 275.0)))

(event Input|AxisEvents|InputAxisMoveForward
  (params (AxisValue :type Float%20%28single-precision%29))
  (Pawn|Input|AddMovementInput (Math|Vector|GetForwardVector (Transformation|GetActorRotation)) (* AxisValue 4.0) false))

(event Input|AxisEvents|InputAxisMoveRight
  (params (AxisValue :type Float%20%28single-precision%29))
  (Pawn|Input|AddMovementInput (Math|Vector|GetRightVector (Transformation|GetActorRotation)) (* AxisValue 1.0) false))

(event Input|AxisEvents|InputAxisTurn
  (params (AxisValue :type Float%20%28single-precision%29))
  (Pawn|Input|AddControllerYawInput (* AxisValue (Variables|Default|GetMouseSensitivity))))

(event Input|AxisEvents|InputAxisLookUp
  (params (AxisValue :type Float%20%28single-precision%29))
  (Pawn|Input|AddControllerPitchInput (* AxisValue (Variables|Default|GetMouseSensitivity))))

(fn ConstructionScript)