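; Handler for the WOM ride that spawns trains evenly spaced along a spline track and manages player boarding.
; Tick finds the train at the entrance and prompts when the player overlaps one of its cars; Interact toggles riding.
; Riding snaps an attachment to the car seat, blends the view to this actor and offsets WedwayCam by control-rotation delta.
; Once the car climbs past a height threshold, it opens WoMRidePlayer_Ride and exits, teleporting the player.
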(event Custom|SwitchToFirstPerson
  (params (TransitionTime :type Float%20%28single-precision%29))
  (CallFunction|ToggleWedwayView (Variables|Default|GetTrainNum) (Variables|Default|GetCarNum) TransitionTime true))

(event EventBeginPlay
  (for _index (range 0 (- (Variables|Default|GetTrainsAmount) 1))
    (bind _returnvalue (Game|SpawnActorfromClass "/Game/Blueprints/WOMTest/WOMTrain_BP3.WOMTrain_BP3_C" (Math|Transform|MakeTransform "0, 0, 0" "0, 0, 0" "1,1,1") "Undefined" 0 0))
    (Utilities|Array|Add (Variables|Default|GetTrains) _returnvalue)
    (Class|VehicleTrain|StartTrain _returnvalue (Variables|Default|GetTrack) (* _index (/ (Spline|GetSplineLength (Variables|/Script/FP82MasterNew.TrackBase|GetSpline (Variables|Default|GetTrack))) (Math|Conversions|ToFloat(Integer) (Variables|Default|GetTrainsAmount)))) 2.5e+02))
  (Variables|Default|SetComplete? true))

(event EventTick
  (params (DeltaSeconds :type Float%20%28single-precision%29))
  (bind _returnvalue (Game|GetPlayerController 0))
  (bind _trains (Variables|Default|GetTrains))
  (bind _returnvalue_2 (Pawn|GetControlRotation _returnvalue :!class /Script/Engine.Controller))
  (if (Variables|Default|GetComplete?)
    (if (Variables|Default|GetCharacterRiding)
      (bind _output_get (Variables|Default|SetCurrentControlRotation (Math|Rotator|MakeRotator (* (- (.roll (Variables|Default|GetOriginalControlRotation)) (.roll _returnvalue_2)) -1.0) (* (- (.pitch (Variables|Default|GetOriginalControlRotation)) (.pitch _returnvalue_2)) -1.0) (* (- (.yaw (Variables|Default|GetOriginalControlRotation)) (.yaw _returnvalue_2)) -1.0))))
      (Transformation|SetRelativeRotation (Variables|Default|GetWedwayCam) _output_get false false)
      (if (> (.z (Transformation|GetActorLocation (Utilities|Array|Get(acopy) (Variables|/Script/FP82MasterNew.VehicleTrain|GetRideVehicles (Utilities|Array|Get(acopy) (Variables|Default|GetTrains) (Variables|Default|GetTrainNum))) (Variables|Default|GetCarNum)))) 9.2e+02)
        (bind _returnvalue_3 (UserInterface|CreateWidget "/Game/Assets/Widgets/WoMRidePlayer_Ride.WoMRidePlayer_Ride_C"))
        (UserInterface|Viewport|AddtoViewport _returnvalue_3 0)
        (CallFunction|ToggleWedwayView 0 0 0.0 false))
      (else
        (for (_array_element _array_index) _trains
          (bind _returnvalue_4 (Actor|GetActorOfClass "/Game/Blueprints/WOM/WOM_Entrance_Overlap.WOM_Entrance_Overlap_C"))
          (if (and (Utilities|IsValid _returnvalue_4) (Utilities|IsValid (Utilities|Array|Get(acopy) (Variables|/Script/FP82MasterNew.VehicleTrain|GetRideVehicles _array_element))))
            (if (and (Collision|IsOverlappingActor _returnvalue_4 (Utilities|Array|Get(acopy) (Variables|/Script/FP82MasterNew.VehicleTrain|GetRideVehicles _array_element)) :!class /Script/Engine.Actor) (> (Utilities|Array|Length _trains) 0))
              (Variables|Default|SetTrainNum _array_index)
              (for (_array_element_2 _array_index_2) (Variables|/Script/FP82MasterNew.VehicleTrain|GetRideVehicles _array_element)
                (bind _output_get_2 (Variables|Default|SetOverlap? (Collision|IsOverlappingActor (Game|GetPlayerCharacter 0) _array_element_2 :!class /Script/Engine.Actor)))
                (if _output_get_2
                  (Variables|Default|SetCarNum _array_index_2)
                  (Variables|Default|SetOriginalControlRotation (Pawn|GetControlRotation (Game|GetPlayerController 0) :!class /Script/Engine.Controller))
                  (Variables|Default|SetCurrentControlRotation (Math|Rotator|MakeRotator 0.0 0.0 0.0))
                  (bind _returnvalue_5 (UserInterface|CreateWidget "/Game/Assets/Widgets/Info_Widget.Info_Widget_C" 0 "Press Z to Ride"))
                  (UserInterface|Viewport|AddtoViewport _returnvalue_5 0))))))))))

(event Input|ActionEvents|InputActionInteract
  (params (Key :type Key%20Structure :default "None"))
  (:Pressed
    (if (Variables|Default|GetOverlap?)
      (CallFunction|SwitchtoFirstPerson 2.0))))

(fn ConstructionScript)

(fn ToggleWedwayView
  (params (TrainNum :type Integer) (CarNum :type Integer) (TransitionTime :type Float%20%28single-precision%29) (OrigSitting :type Boolean))
  (bind _returnvalue (Game|GetPlayerController 0))
  (bind _foundwidgets (Widget|GetAllWidgetsOfClass "/Game/Assets/Widgets/Info_Widget.Info_Widget_C" true))
  (Widget|RemovefromParent _foundwidgets)
  (Utilities|FlowControl|Sequence
    (:then_0
      (bind _asdefault_character (Utilities|Casting|CastToDefaultCharacter (Game|Player|GetPlayerPawn 0)))
      (Variables|Default|SetDefaultCharacterRef _asdefault_character))
    (:then_1
      (if (Variables|Default|GetCharacterRiding)
        (Pawn|SetControlRotation (Game|GetPlayerController 0) (Variables|Default|GetOriginalControlRotation))
        (Transformation|Teleport (Game|GetPlayerCharacter 0) "20250.000000,9260.000000,200.000000" "0, 0, 0")
        (Game|Player|SetViewTargetwithBlend (Game|GetPlayerController 0) (Game|Player|GetPlayerPawn 0) TransitionTime "VTBlend_Linear" 0.0 false)
        (Variables|Default|SetCharacterRiding false)
        (Input|DisableInput (Game|GetPlayerController 0))
        (bind _asfp82game_instance (Utilities|Casting|CastToFP82GameInstance (Game|GetGameInstance)))
        (Variables|/Game/Assets/Blueprints/FP82GameInstance.FP82GameInstance_C|SetRidingWOM _asfp82game_instance false)
        (else
          (bind _aswomcar_new__bp (Utilities|Casting|CastToWOMCar_New+BP (Utilities|Array|Get(acopy) (Variables|/Script/FP82MasterNew.VehicleTrain|GetRideVehicles (Utilities|Array|Get(acopy) (Variables|Default|GetTrains) TrainNum)) CarNum)))
          (Transformation|AttachComponentToComponent self (Variables|/Game/Blueprints/WOMTest/WOMCar_New+BP.WOMCar_New+BP_C|GetSittingPositionFront _aswomcar_new__bp) "None" "SnapToTarget" "SnapToTarget" "KeepRelative" true)
          (Game|Player|SetViewTargetwithBlend _returnvalue self TransitionTime "VTBlend_Linear" 0.0 false)
          (Variables|Default|SetOriginalControlRotation (Pawn|GetControlRotation _returnvalue :!class /Script/Engine.Controller))
          (Variables|Default|SetCharacterRiding true)
          (bind _returnvalue_2 (UserInterface|CreateWidget "/Game/Assets/Widgets/Info_Widget.Info_Widget_C" 0 "Press Z to Skip Ride"))
          (UserInterface|Viewport|AddtoViewport _returnvalue_2 0)
          (Default|Fade5 _returnvalue_2)
          (Input|EnableInput (Game|GetPlayerController 0))
          (bind _asfp82game_instance_2 (Utilities|Casting|CastToFP82GameInstance (Game|GetGameInstance)))
          (Variables|/Game/Assets/Blueprints/FP82GameInstance.FP82GameInstance_C|SetRidingWOM _asfp82game_instance_2 true))))))