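; WOMTrain_BP3 is a ride train that spawns and manages a set of WOMCar_NewBP vehicles and controls their shared speed.
; On BeginPlay it spawns cars according to CarAmount, links each back to itself with smooth rotation on, and starts in Travel mode.
; ChangeSpeed maps each new mode to a target speed, and a timeline curve eases CurrentSpeed toward it.
; Actual movement is not handled in this Blueprint.
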(event Custom|ChangeSpeed
  (params (SpeedType :type ETrainMode%20Enum :default "Idle") (SpeedScalar :type Float%20%28single-precision%29))
  (if (Utilities|Enum|NotEqual(Enum) (Variables|Default|GetCurrentMode) SpeedType)
    (Utilities|FlowControl|Sequence
      (:then_0
        (Variables|Default|SetStartSpeed (Variables|Default|GetCurrentSpeed)))
      (:then_1
        (bind _output_get (Variables|Default|SetCurrentMode SpeedType))
        (switch Utilities|FlowControl|Switch|SwitchonETrainMode _output_get
          (:Idle
            (bind _output_get_2 (Variables|Default|SetTargetSpeed 0.0)))
          (:Travel
            (Variables|Default|SetTargetSpeed (Variables|Default|GetMaxSpeed)))
          (:Loading
            (Variables|Default|SetTargetSpeed (Variables|Default|GetMinSpeed)))
          (:SpeedScalar
            (Variables|Default|SetTargetSpeed (* (Variables|Default|GetMaxSpeed) SpeedScalar)))))
      (:then_2
        (bind _newtrack_0 (Timeline|Acceleration%20Curve PlayFromStart)
          (:Update
            (Variables|Default|SetCurrentSpeed (Math|Float|Lerp (Variables|Default|GetStartSpeed) (Variables|Default|GetTargetSpeed) _newtrack_0))))))))

(event EventBeginPlay
  (Utilities|FlowControl|Sequence
    (:then_0
      (Utilities|Array|Clear (Variables|Default|GetRideVehicles)))
    (:then_1
      (for _index (range 0 (Variables|Default|GetCarAmount))
        (bind _returnvalue (Game|SpawnActorfromClass "/Game/Blueprints/WOMTest/WOMCar_New+BP.WOMCar_New+BP_C" (Math|Transform|MakeTransform "0, 0, 0" "0, 0, 0" "1,1,1") "Undefined" 0 0))
        (Variables|/Script/FP82MasterNew.RideVehicle|SetSmoothRotation _returnvalue true)
        (Variables|/Game/Blueprints/WOMTest/WOMCar_New+BP.WOMCar_New+BP_C|SetVehicleTrain _returnvalue self)
        (Utilities|Array|Add (Variables|Default|GetRideVehicles) _returnvalue))
      (CallFunction|ChangeSpeed "Travel" 0.0))))

(fn ConstructionScript)